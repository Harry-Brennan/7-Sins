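; BP_NPC is a computer-controlled card player in the bar's card games.
; It keeps its cards in a current-hand component, with events to add and remove cards.
; On its turn it prints its name, waits briefly, then checks the bar game mode's active game.
; For I Doubt It, it always plays the first card in hand by passing it to that game's manager to end the turn.
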(event EventAddCardtoHand
  (params (Card :type BP%20Card%20Object%20Reference))
  (Utilities|Array|Add (Variables|/Game/Shared_Game_Mechanics/BPC_CurrentHand.BPC_CurrentHand_C|GetCurrent%20Hand (Variables|Default|GetBPC_CurrentHand)) Card))

(event EventRemoveCardfromHand
  (params (Card :type BP%20Card%20Object%20Reference))
  (Utilities|Array|RemoveItem (Variables|/Game/Shared_Game_Mechanics/BPC_CurrentHand.BPC_CurrentHand_C|GetCurrent%20Hand (Variables|Default|GetBPC_CurrentHand)) Card))

(event EventBeginPlay
  (bind _asgm_bar (Utilities|Casting|CastToGM_Bar (Game|GetGameMode)))
  (Variables|Default|SetAs%20GM%20Bar _asgm_bar))

(event EventTakeTurn
  (Development|PrintString (Utilities|String|Append "Current turn: " (Utilities|GetDisplayName self)))
  (Utilities|FlowControl|Delay 1.0)
  (switch Utilities|FlowControl|Switch|SwitchonEnum_All_Game_Names (Variables|/Game/Modes_Instances/Modes/GM_Bar.GM_Bar_C|GetCurrent%20Playing%20Game (Variables|Default|GetAs%20GM%20Bar))
    (:NewEnumerator0
      (bind _returnvalue (Actor|GetActorOfClass "/Game/Main_Game_Managers/I_Doubt_It/BP_I_Doubt_It_Game_Manager.BP_I_Doubt_It_Game_Manager_C"))
      (Default|EndPlayerTurn _returnvalue self (Utilities|Array|MakeArray (Utilities|Array|Get(acopy) (Variables|/Game/Shared_Game_Mechanics/BPC_CurrentHand.BPC_CurrentHand_C|GetCurrent%20Hand (Variables|Default|GetBPC_CurrentHand))))))))

(fn ConstructionScript)