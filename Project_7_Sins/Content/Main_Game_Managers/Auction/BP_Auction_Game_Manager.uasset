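; Game manager for the Auction card game, where the player and tagged NPCs bid cards to win auctioned cards.
; It seats participants at tagged target points and works through the card dealer, turn manager and tagged piles.
; EndRound totals played cards, including special-card effects, then awards the lot or replays among tied players.
; An empty main pile triggers final scoring of won cards; fading world widgets mark active players and draws.
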(event Custom|Fade%20Out%20Turn%20Indicator
  (bind _values (Utilities|Map|Values (Variables|Players+Positions|GetPlaying%20Characters%20->%20Can%20Play%20Round)))
  (bind _alpha (Timeline|Fade%20Out%20Round%20Indicator%20Timeline PlayFromStart)
    (:Update
      (for (_array_element _array_index) (Variables|Widgets|GetTurn%20Indicators)
        (if (not (Utilities|Array|Get(acopy) _values _array_index))
          (Class|WidgetComponent|SetTintColorandOpacity _array_element (Math|Color|Lerp(LinearColor) "(R=1.000000,G=1.000000,B=1.000000,A=1.000000)" "(R=1.000000,G=1.000000,B=1.000000,A=0.000000)" _alpha)))))
    (:Finished
      (for (_array_element_2 _array_index_2) (Variables|Widgets|GetTurn%20Indicators)
        (if (not (Utilities|Array|Get(acopy) _values _array_index_2))
          (Rendering|SetVisibility _array_element_2 false false)
          (Class|WidgetComponent|SetTintColorandOpacity _array_element_2 "(R=1.000000,G=1.000000,B=1.000000,A=1.000000)"))))))

(event Custom|Fade%20Out%20Draw%20Indicator
  (bind _draw_widget (Variables|Widgets|GetDraw%20Widget))
  (bind _alpha (Timeline|Fade%20Out%20Draw%20Indicator%20Timeline PlayFromStart)
    (:Update
      (Class|WidgetComponent|SetTintColorandOpacity (Variables|Widgets|GetDraw%20Widget) (Math|Color|Lerp(LinearColor) "(R=1.000000,G=1.000000,B=1.000000,A=1.000000)" "(R=1.000000,G=1.000000,B=1.000000,A=0.000000)" _alpha)))
    (:Finished
      (Rendering|SetVisibility _draw_widget false false)
      (Class|WidgetComponent|SetTintColorandOpacity _draw_widget "(R=1.000000,G=1.000000,B=1.000000,A=1.000000)"))))

(event EventBeginPlay
  (Utilities|SetPlayingPositionsVariables
    (:Done
      (Utilities|SetReferences)
      (Utilities|SetupWidgets))))

(fn ConstructionScript)

(fn SetupAuction
  ;[0 0 0] Setup auction and cards
  (bind _returnvalue (Actor|GetActorOfClass "/Game/Player/BP_Player.BP_Player_C"))
  (Utilities|Map|Add (Variables|Players+Positions|GetPlaying%20Characters%20->%20Can%20Play%20Round) _returnvalue true)
  (bind _outactors (Actor|GetAllActorsOfClasswithTag "/Game/NPCs/BP_NPC.BP_NPC_C" "Auction_Participant"))
  (for _array_element _outactors
    (Utilities|Map|Add (Variables|Players+Positions|GetPlaying%20Characters%20->%20Can%20Play%20Round) _array_element true))
  (Default|SetupCards (Variables|References|GetCard%20Dealer%20Reference) "NewEnumerator1")
  (Main|MoveCharacters)
  (Widgets|SetupTurnIndicators))

(fn StartAuction
  ;[0 0 0] Start various aspects of the game
  (bind _keys (Utilities|Map|Keys (Variables|Players+Positions|GetPlaying%20Characters%20->%20Can%20Play%20Round)))
  (Default|DealCards (Variables|References|GetCard%20Dealer%20Reference) "NewEnumerator1" _keys)
  (Default|SetupMainGame (Variables|References|GetTurn%20Manager%20Reference) "NewEnumerator1" _keys)
  (Default|StartFirstTurn (Variables|References|GetTurn%20Manager%20Reference) "NewEnumerator1"))

(fn CheckifGameOver
  (if (Utilities|Array|IsEmpty (Variables|/Game/Shared_Game_Mechanics/Cards/BP_CardPile.BP_CardPile_C|GetCardsInPile (Variables|References|GetAuction%20Main%20Card%20Pile)))
    (GameOver|AuctionGameOver)
    (else
      (Main|NextRound))))

(fn EndRound
  (bind _keys (Utilities|Map|Keys (Variables|Players+Positions|GetPlaying%20Characters%20->%20Can%20Play%20Round)))
  (for (_array_element _array_index) _keys
    (bind _output_get (LocalVariables|SetCurrent%20Loop%20Current%20Hand (Variables|/Game/Shared_Game_Mechanics/BPC_CurrentHand.BPC_CurrentHand_C|GetSelected%20Cards (Actor|GetComponentbyClass _array_element "/Game/Shared_Game_Mechanics/BPC_CurrentHand.BPC_CurrentHand_C"))))
    (for _array_element_2 _output_get
      (bind _card_info (Default|GetCardInfo _array_element_2))
      (if (> (.NumericalValue (Utilities|Struct|BreakStruct_Card _card_info)) 13)
        (bind _card_value (UniqueCard|UnqiueCardAction (Utilities|Select :Index (.CardName (Utilities|Struct|BreakStruct_Card _card_info)) :NewEnumerator0 "NewEnumerator0" :NewEnumerator1 "NewEnumerator0" :NewEnumerator2 "NewEnumerator0" :NewEnumerator3 "NewEnumerator0" :NewEnumerator4 "NewEnumerator0" :NewEnumerator5 "NewEnumerator0" :NewEnumerator6 "NewEnumerator0" :NewEnumerator7 "NewEnumerator0" :NewEnumerator8 "NewEnumerator0" :NewEnumerator9 "NewEnumerator0" :NewEnumerator10 "NewEnumerator0" :NewEnumerator11 "NewEnumerator0" :NewEnumerator12 "NewEnumerator0" :NewEnumerator13 "NewEnumerator0" :NewEnumerator14 "NewEnumerator1" :NewEnumerator15 "NewEnumerator2" :NewEnumerator61 "NewEnumerator3" :NewEnumerator62 "NewEnumerator7" :NewEnumerator63 "NewEnumerator3" :NewEnumerator64 "NewEnumerator6" :NewEnumerator66 "NewEnumerator5") _array_index))
        (Utilities|Array|SetArrayElem (LocalVariables|GetPlayer%20Scores) _array_index _card_value)
        (else
          (Utilities|Array|SetArrayElem (LocalVariables|GetPlayer%20Scores) _array_index (+ (Utilities|Array|Get(acopy) (LocalVariables|GetPlayer%20Scores) _array_index) (.NumericalValue (Utilities|Struct|BreakStruct_Card _card_info))))))
      (Default|RemoveCardfromPlayerHand (Variables|References|GetCard%20Dealer%20Reference) _array_element _array_element_2)
      (Default|AddCardtoPile (Variables|References|GetCard%20Dealer%20Reference) _array_element_2 (Utilities|Array|Get(acopy) (Variables|References|GetPlayed%20Card%20Piles) _array_index) false)))
  (bind _keys_2 (Utilities|Map|Keys (Variables|Players+Positions|GetPlaying%20Characters%20->%20Can%20Play%20Round)))
  (for _array_element_3 _keys_2
    (Default|ClearSelectedCards (Actor|GetComponentbyClass _array_element_3 "/Game/Shared_Game_Mechanics/BPC_CurrentHand.BPC_CurrentHand_C")))
  (for (_array_element_4 _array_index_2) (LocalVariables|GetPlayer%20Scores)
    (Development|PrintString (Utilities|String|Append "CURRENT ROUND SCORE FOR : " (Utilities|GetDisplayName (Utilities|Array|Get(acopy) _keys_2 _array_index_2)) " IS " (Utilities|String|ToString(Integer) _array_element_4)) true true "(R=0.000000,G=0.660000,B=1.000000,A=1.000000)" 1e+02)
    (if (> _array_element_4 (LocalVariables|GetHighest%20Score))
      (LocalVariables|SetHighest%20Score _array_element_4)))
  (for (_array_element_5 _array_index_3) (LocalVariables|GetPlayer%20Scores)
    (if (== _array_element_5 (LocalVariables|GetHighest%20Score))
      (Utilities|Array|Add (LocalVariables|GetDrawing%20Indexes) _array_index_3)))
  (if (> (Utilities|Array|Length (LocalVariables|GetDrawing%20Indexes)) 1)
    (Development|PrintString "ROUND DRAW")
    (bind _keys_3 (Utilities|Map|Keys (Variables|Players+Positions|GetPlaying%20Characters%20->%20Can%20Play%20Round)))
    (Widgets|UpdateDrawIndicator)
    (for (_array_element_6 _array_index_4) _keys_3
      (if (Utilities|Array|ContainsItem (LocalVariables|GetDrawing%20Indexes) _array_index_4)
        (Development|PrintString (Utilities|String|Append (Utilities|GetDisplayName _array_element_6) " IS A DRAWING PLAYER"))
        (else
          (Utilities|Map|Add (Variables|Players+Positions|GetPlaying%20Characters%20->%20Can%20Play%20Round) _array_element_6 false))))
    (Widgets|UpdateTurnIndicators)
    (EndRound|NPCSelectAllCardsforRound)
    (bind _returnvalue (Actor|GetActorOfClass "/Game/Player/BP_Player.BP_Player_C"))
    (if (Utilities|Array|ContainsItem (LocalVariables|GetDrawing%20Indexes) (Utilities|Array|FindItem _keys_3 _returnvalue))
      (Utilities|Time|SetTimerbyFunctionName _returnvalue "Take Turn" 1.0)
      (else
        (Utilities|Time|SetTimerbyFunctionName 0 "End Round" 2.0)))
    (else
      (LocalVariables|SetWon%20Card (Utilities|Array|Get(acopy) (Variables|/Game/Shared_Game_Mechanics/Cards/BP_CardPile.BP_CardPile_C|GetCardsInPile (Variables|References|GetAuctioning%20Pile))))
      (bind _keys_4 (Utilities|Map|Keys (Variables|Players+Positions|GetPlaying%20Characters%20->%20Can%20Play%20Round)))
      (Utilities|Map|Add (Variables|WonCards|GetWon%20Card%20->%20Player) (LocalVariables|GetWon%20Card) (Utilities|Array|Get(acopy) _keys_4 (Utilities|Array|FindItem (LocalVariables|GetPlayer%20Scores) (LocalVariables|GetHighest%20Score))))
      (Development|PrintString (Utilities|String|Append "WON PLAYER FOR ROUND : " (Utilities|GetDisplayName (Utilities|Array|Get(acopy) _keys_4 (Utilities|Array|FindItem (LocalVariables|GetPlayer%20Scores) (LocalVariables|GetHighest%20Score))))) true true "(R=0.000000,G=0.660000,B=1.000000,A=1.000000)" 1e+02)
      (Default|RemoveCardfromPile (Variables|References|GetCard%20Dealer%20Reference) (LocalVariables|GetWon%20Card) (Variables|References|GetAuctioning%20Pile))
      (Default|AddCardtoPile (Variables|References|GetCard%20Dealer%20Reference) (LocalVariables|GetWon%20Card) (Utilities|Array|Get(acopy) (Variables|References|GetWon%20Card%20Piles) (Utilities|Array|FindItem (LocalVariables|GetPlayer%20Scores) (LocalVariables|GetHighest%20Score))) false)
      (bind _keys_5 (Utilities|Map|Keys (Variables|Players+Positions|GetPlaying%20Characters%20->%20Can%20Play%20Round)))
      (for _array_element_7 _keys_5
        (Utilities|Map|Add (Variables|Players+Positions|GetPlaying%20Characters%20->%20Can%20Play%20Round) _array_element_7 true))
      (Main|NextRound))))

(fn CalculatePlayerHandValues
  (bind _won_card____player (Variables|WonCards|GetWon%20Card%20->%20Player))
  (bind _player____score (LocalVariables|GetPlayer%20->%20Score))
  (bind _keys (Utilities|Map|Keys _won_card____player))
  (for _array_element _keys
    (bind _card_info (Default|GetCardInfo _array_element))
    (Utilities|Map|Add (LocalVariables|GetPlayer%20->%20Score) (.Value (Utilities|Map|Find _won_card____player _array_element)) (Utilities|Select :Index (Utilities|Struct|BreakStruct_Card _card_info) :NewEnumerator0 (Class|KismetSystemLibrary|MakeLiteralInteger 4) :NewEnumerator1 0 :NewEnumerator2 0 :NewEnumerator3 0 :NewEnumerator4 0 :NewEnumerator5 0 :NewEnumerator6 0 :NewEnumerator7 0 :NewEnumerator8 0 :NewEnumerator9 0 :NewEnumerator10 (Class|KismetSystemLibrary|MakeLiteralInteger 3) :NewEnumerator11 (Class|KismetSystemLibrary|MakeLiteralInteger 2) :NewEnumerator12 (Class|KismetSystemLibrary|MakeLiteralInteger 1) :NewEnumerator13 0 :NewEnumerator14 0 :NewEnumerator15 0 :NewEnumerator61 0 :NewEnumerator62 0 :NewEnumerator63 0 :NewEnumerator64 0 :NewEnumerator66 0)))
  (bind _keys_2 (Utilities|Map|Keys _player____score))
  (for _array_element_2 _keys_2
    (if (> (.Value (Utilities|Map|Find _player____score _array_element_2)) (LocalVariables|GetHighest%20Score))
      (LocalVariables|SetHighest%20Score (.Value (Utilities|Map|Find _player____score _array_element_2)))
      (LocalVariables|SetHighest%20Scoring%20Player _array_element_2)))
  (return (LocalVariables|GetHighest%20Scoring%20Player)))

(fn MoveCharacters
  (bind _keys (Utilities|Map|Keys (Variables|Players+Positions|GetPlaying%20Characters%20->%20Can%20Play%20Round)))
  (for (_array_element _array_index) _keys
    (Transformation|SetActorLocationAndRotation _array_element (Utilities|Select :Index _array_index :Option%200 (Transformation|GetActorLocation (Variables|Players+Positions|GetPlayer%20Position)) :Option%201 (Transformation|GetActorLocation (Variables|Players+Positions|GetOpponent%201%20Position)) :Option%202 (Transformation|GetActorLocation (Variables|Players+Positions|GetOpponent%202%20Position)) :Option%203 (Transformation|GetActorLocation (Variables|Players+Positions|GetOpponent%203%20Position))) (Utilities|Select :Index _array_index :Option%200 (Transformation|GetActorRotation (Variables|Players+Positions|GetPlayer%20Position)) :Option%201 (Transformation|GetActorRotation (Variables|Players+Positions|GetOpponent%201%20Position)) :Option%202 (Transformation|GetActorRotation (Variables|Players+Positions|GetOpponent%202%20Position)) :Option%203 (Transformation|GetActorRotation (Variables|Players+Positions|GetOpponent%203%20Position))))))

(fn AuctionGameOver
  (bind _highest_scored_player (GameOver|CalculatePlayerHandValues))
  (Development|PrintString (Utilities|String|Append "AUCTION GAME OVER, WINNER: " (Utilities|GetDisplayName _highest_scored_player))))

(fn NextRound
  (bind _auction_main_card_pile (Variables|References|GetAuction%20Main%20Card%20Pile))
  (bind _cardsinpile (Variables|/Game/Shared_Game_Mechanics/Cards/BP_CardPile.BP_CardPile_C|GetCardsInPile _auction_main_card_pile))
  (bind _returnvalue (Utilities|Array|LastIndex _cardsinpile))
  (bind _output (Utilities|Array|Get(acopy) _cardsinpile _returnvalue))
  (LocalVariables|SetCard%20to%20Auction _output)
  (Default|RemoveCardfromPile (Variables|References|GetCard%20Dealer%20Reference) _output (Variables|References|GetAuction%20Main%20Card%20Pile))
  (Default|AddCardtoPile (Variables|References|GetCard%20Dealer%20Reference) (LocalVariables|GetCard%20to%20Auction) (Variables|References|GetAuctioning%20Pile) false)
  (Widgets|UpdateTurnIndicators)
  (EndRound|NPCSelectAllCardsforRound)
  (bind _returnvalue_2 (Actor|GetActorOfClass "/Game/Player/BP_Player.BP_Player_C"))
  (Utilities|Time|SetTimerbyFunctionName _returnvalue_2 "Take Turn" 1.0))

(fn NPCSelectAllCardsforRound
  (bind _keys (Utilities|Map|Keys (Variables|Players+Positions|GetPlaying%20Characters%20->%20Can%20Play%20Round)))
  (for _array_element _keys
    (if (.Value (Utilities|Map|Find (Variables|Players+Positions|GetPlaying%20Characters%20->%20Can%20Play%20Round) _array_element))
      (if (Utilities|DoesObjectImplementInterface _array_element "/Game/NPCs/BPI_NPC_Opponent.BPI_NPC_Opponent_C")
        (Class|BPIPlayingCharacter|TakeTurn(Message) _array_element)))))

(fn UpdateTurnIndicators
  (bind _values (Utilities|Map|Values (Variables|Players+Positions|GetPlaying%20Characters%20->%20Can%20Play%20Round)))
  (for (_array_element _array_index) _values
    (if _array_element
      (Rendering|SetVisibility (Utilities|Array|Get(acopy) (Variables|Widgets|GetTurn%20Indicators) _array_index) true false)))
  (if (Utilities|Array|ContainsItem _values false)
    (CallFunction|FadeOutTurnIndicator)))

(fn SetupTurnIndicators
  (bind _playing_characters____can_play_round (Variables|Players+Positions|GetPlaying%20Characters%20->%20Can%20Play%20Round))
  (bind _values (Utilities|Map|Values _playing_characters____can_play_round))
  (bind _keys (Utilities|Map|Keys _playing_characters____can_play_round))
  (for (_array_element _array_index) _values
    (if _array_element
      (Transformation|SetWorldLocationAndRotation (Utilities|Array|Get(acopy) (Variables|Widgets|GetTurn%20Indicators) _array_index) (+ (Transformation|GetActorLocation (Utilities|Array|Get(acopy) _keys _array_index)) "0.000000,0.000000,180.000000") (Math|Rotator|FindLookatRotation (Transformation|GetActorLocation (Utilities|Array|Get(acopy) _keys _array_index)) (Transformation|GetActorLocation (Variables|References|GetAuctioning%20Pile))) false false))))

(fn UpdateDrawIndicator
  (bind _auction_main_card_pile (Variables|References|GetAuction%20Main%20Card%20Pile))
  (bind _returnvalue (Transformation|GetActorLocation _auction_main_card_pile))
  (bind _returnvalue_2 (+ _returnvalue "0.000000,0.000000,100.000000"))
  (bind _returnvalue_3 (Actor|GetActorOfClass "/Game/Player/BP_Player.BP_Player_C"))
  (Transformation|SetWorldLocationAndRotation (Variables|Widgets|GetDraw%20Widget) _returnvalue_2 (Math|Rotator|FindLookatRotation _returnvalue_2 (Transformation|GetActorLocation _returnvalue_3)) false false)
  (Rendering|SetVisibility (Variables|Widgets|GetDraw%20Widget) true false)
  (CallFunction|FadeOutDrawIndicator))

(fn UnqiueCardAction
  (params (Card%20Played :type Enum_Unique_Card_Names%20Enum :default "NewEnumerator0") (Player%20Index :type Integer))
  (bind _played_card_piles (Variables|References|GetPlayed%20Card%20Piles))
  (bind _all_played_cards (LocalVariables|GetAll%20Played%20Cards))
  (bind _output (Utilities|Array|Get(acopy) _played_card_piles Player%20Index))
  (bind _cardsinpile (Variables|/Game/Shared_Game_Mechanics/Cards/BP_CardPile.BP_CardPile_C|GetCardsInPile _output))
  (Development|PrintString "UNIQUE CARD ACTION AUCTION" true true "(R=0.000000,G=0.660000,B=1.000000,A=1.000000)" 1e+02)
  (switch Utilities|FlowControl|Switch|SwitchonEnum_Unique_Card_Names Card%20Played
    (:NewEnumerator0
      ;[0 0 0] Joker - Duplicate previous round's played card for this round
      (bind _card_info (Default|GetCardInfo (Utilities|Array|Get(acopy) _cardsinpile (Utilities|Array|LastIndex _cardsinpile))))
      (if (Utilities|Enum|Equal(Enum) (.Suit (Utilities|Struct|BreakStruct_Card _card_info)) "NewEnumerator4")
        (return 10)
        (else
          (return (.NumericalValue (Utilities|Struct|BreakStruct_Card _card_info))))))
    (:NewEnumerator1
      ;[0 0 0] Devil - steal a won card from a random player
      (bind _output_get (LocalVariables|SetWon%20Card%20Piles%20Excluding%20Played (Variables|References|GetWon%20Card%20Piles)))
      (Utilities|Array|RemoveIndex _output_get Player%20Index)
      (bind _output_get_2 (LocalVariables|SetWon%20Card%20to%20Move (.OutItem (Utilities|Array|Random (Variables|/Game/Shared_Game_Mechanics/Cards/BP_CardPile.BP_CardPile_C|GetCardsInPile (.OutItem (Utilities|Array|Random (LocalVariables|GetWon%20Card%20Piles%20Excluding%20Played))))))))
      (Default|RemoveCardfromPile (Variables|References|GetCard%20Dealer%20Reference) _output_get_2 (.OutItem (Utilities|Array|Random (LocalVariables|GetWon%20Card%20Piles%20Excluding%20Played))))
      (Default|AddCardtoPile (Variables|References|GetCard%20Dealer%20Reference) (LocalVariables|GetWon%20Card%20to%20Move) (Utilities|Array|Get(acopy) (Variables|References|GetWon%20Card%20Piles) Player%20Index) false)
      (return 0))
    (:NewEnumerator2
      ;[0 0 0] Angel - becomes the highest scoring card of the round forcing a draw to occur
      (Utilities|Map|Add (Variables|UniqueCard|GetPlayer%20->%20Angel%20Active) 0 true)
      (return 0))
    (:NewEnumerator3
      ;[0 0 0] War - stop a player from playing any cards in the next turn
      (Utilities|Map|Add (Variables|UniqueCard|GetPlayer%20->%20War%20Active) 0 true)
      (return 0))
    (:NewEnumerator4
      ;[0 0 0] Pestilence - reduces the value of every card played in the next turn by 1
      (Variables|UniqueCard|SetPestilence%20Active false)
      (return 0))
    (:NewEnumerator5
      ;[0 0 0] Conquest - allows the player to play two cards in the next turn
      (Utilities|Map|Add (Variables|UniqueCard|GetPlayer%20->%20Conquest%20Active) 0 false)
      (return 0))
    (:NewEnumerator6
      ;[0 0 0] Famine - swaps a random player's hand with another random player's hand
      (bind _keys (Utilities|Map|Keys (Variables|Players+Positions|GetPlaying%20Characters%20->%20Can%20Play%20Round)))
      (bind _output_get_3 (LocalVariables|SetFamine%20Players%20Excluding%20Played (Variables|/Game/Shared_Game_Mechanics/Turn_Taking/BP_Turn_Manager.BP_Turn_Manager_C|GetPlaying%20Characters (Variables|References|GetTurn%20Manager%20Reference))))
      (Utilities|Array|RemoveItem _output_get_3 (Utilities|Array|Get(acopy) _keys Player%20Index))
      (bind _output_get_4 (LocalVariables|SetFamine%20Player%20Swap%201 (.OutItem (Utilities|Array|Random (LocalVariables|GetFamine%20Players%20Excluding%20Played)))))
      (Utilities|Array|RemoveItem (LocalVariables|GetFamine%20Players%20Excluding%20Played) _output_get_4)
      (LocalVariables|SetFamine%20Player%20Swap%202 (.OutItem (Utilities|Array|Random (LocalVariables|GetFamine%20Players%20Excluding%20Played))))
      (LocalVariables|SetFamine%20Temp%20Card%20Hand (Variables|/Game/Shared_Game_Mechanics/BPC_CurrentHand.BPC_CurrentHand_C|GetCurrent%20Hand (Actor|GetComponentbyClass (LocalVariables|GetFamine%20Player%20Swap%201) "/Game/Shared_Game_Mechanics/BPC_CurrentHand.BPC_CurrentHand_C")))
      (Variables|/Game/Shared_Game_Mechanics/BPC_CurrentHand.BPC_CurrentHand_C|SetCurrent%20Hand (Actor|GetComponentbyClass (LocalVariables|GetFamine%20Player%20Swap%201) "/Game/Shared_Game_Mechanics/BPC_CurrentHand.BPC_CurrentHand_C") (Variables|/Game/Shared_Game_Mechanics/BPC_CurrentHand.BPC_CurrentHand_C|GetCurrent%20Hand (Actor|GetComponentbyClass (LocalVariables|GetFamine%20Player%20Swap%202) "/Game/Shared_Game_Mechanics/BPC_CurrentHand.BPC_CurrentHand_C")))
      (bind _hand_spline (Class|BPIPlayingCharacter|GetCurrentHandSpline(Message) (LocalVariables|GetFamine%20Player%20Swap%201)))
      (if (Utilities|DoesObjectImplementInterface (LocalVariables|GetFamine%20Player%20Swap%201) "/Game/NPCs/BPI_NPC_Opponent.BPI_NPC_Opponent_C")
        (Default|UpdateVisibleHand (Actor|GetComponentbyClass (LocalVariables|GetFamine%20Player%20Swap%201) "/Game/Shared_Game_Mechanics/BPC_CurrentHand.BPC_CurrentHand_C") _hand_spline false)
        (else
          (Default|UpdateVisibleHand (Actor|GetComponentbyClass (LocalVariables|GetFamine%20Player%20Swap%201) "/Game/Shared_Game_Mechanics/BPC_CurrentHand.BPC_CurrentHand_C") _hand_spline true (Actor|GetComponentbyClass (LocalVariables|GetFamine%20Player%20Swap%201) "/Script/Engine.CameraComponent"))))
      (Variables|/Game/Shared_Game_Mechanics/BPC_CurrentHand.BPC_CurrentHand_C|SetCurrent%20Hand (Actor|GetComponentbyClass (LocalVariables|GetFamine%20Player%20Swap%202) "/Game/Shared_Game_Mechanics/BPC_CurrentHand.BPC_CurrentHand_C") (LocalVariables|GetFamine%20Temp%20Card%20Hand))
      (bind _hand_spline_2 (Class|BPIPlayingCharacter|GetCurrentHandSpline(Message) (LocalVariables|GetFamine%20Player%20Swap%202)))
      (if (Utilities|DoesObjectImplementInterface (LocalVariables|GetFamine%20Player%20Swap%202) "/Game/NPCs/BPI_NPC_Opponent.BPI_NPC_Opponent_C")
        (Default|UpdateVisibleHand (Actor|GetComponentbyClass (LocalVariables|GetFamine%20Player%20Swap%202) "/Game/Shared_Game_Mechanics/BPC_CurrentHand.BPC_CurrentHand_C") _hand_spline_2 false)
        (else
          (Default|UpdateVisibleHand (Actor|GetComponentbyClass (LocalVariables|GetFamine%20Player%20Swap%202) "/Game/Shared_Game_Mechanics/BPC_CurrentHand.BPC_CurrentHand_C") _hand_spline_2 true (Actor|GetComponentbyClass (LocalVariables|GetFamine%20Player%20Swap%202) "/Script/Engine.CameraComponent"))))
      (return 0))
    (:NewEnumerator7
      ;[0 0 0] Death - deal a random card from each player's played cards pile to a random player - evenly
      (for (_array_element _array_index) (Variables|References|GetPlayed%20Card%20Piles)
        (for _array_element_2 (Variables|/Game/Shared_Game_Mechanics/Cards/BP_CardPile.BP_CardPile_C|GetCardsInPile _array_element)
          (Utilities|Map|Add (LocalVariables|GetAll%20Played%20Cards) _array_element_2 _array_index)))
      (bind _keys_2 (Utilities|Map|Keys (Variables|Players+Positions|GetPlaying%20Characters%20->%20Can%20Play%20Round)))
      (bind _keys_3 (Utilities|Map|Keys _all_played_cards))
      (bind _values (Utilities|Map|Values _all_played_cards))
      (for _index (range 1 (/ (Utilities|Array|Length _keys_3) (Utilities|Array|Length _keys_2)))
        (for _array_element_3 _keys_2
          (Default|RemoveCardfromPile (Variables|References|GetCard%20Dealer%20Reference) (Utilities|Array|Get(acopy) _keys_3 (LocalVariables|GetDealt%20Card%20Index)) (Utilities|Array|Get(acopy) (Variables|References|GetPlayed%20Card%20Piles) (Utilities|Array|Get(acopy) _values (LocalVariables|GetDealt%20Card%20Index))))
          (Default|AddCardtoPlayerHand (Variables|References|GetCard%20Dealer%20Reference) _array_element_3 (Utilities|Array|Get(acopy) _keys_3 (LocalVariables|GetDealt%20Card%20Index)))
          (Math|Integer|IncrementInt (LocalVariables|GetDealt%20Card%20Index)
            (:%20%20
              (Utilities|Array|Add (LocalVariables|GetRe-Dealt%20Played%20Cards) (Utilities|Array|Get(acopy) _keys_3 (LocalVariables|GetDealt%20Card%20Index)))))))
      (bind _keys_4 (Utilities|Map|Keys (LocalVariables|GetAll%20Played%20Cards)))
      (bind _keys_5 (Utilities|Map|Keys (Variables|Players+Positions|GetPlaying%20Characters%20->%20Can%20Play%20Round)))
      (for _array_element_4 _keys_4
        (if (not (Utilities|Array|ContainsItem (LocalVariables|GetRe-Dealt%20Played%20Cards) _array_element_4))
          (Default|AddCardtoPlayerHand (Variables|References|GetCard%20Dealer%20Reference) (Utilities|Array|Get(acopy) _keys_5 (LocalVariables|GetCurrent%20Player%20Deal%20Index)) _array_element_4)
          (Math|Integer|IncrementInt (LocalVariables|GetCurrent%20Player%20Deal%20Index))))
      (return 0))))