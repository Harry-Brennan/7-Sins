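; Game manager for the I Doubt It card game, coordinating setup, dealing, turn hand-off, doubt challenges and game-over checks through the card dealer and turn manager.
; Ending a turn moves played cards to the shared pile, then advances play or prints game over if any hand is empty.
; A doubt compares the last played cards to the expected value, handing the pile to a turn-index-selected player or the doubter.
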(event EventBeginPlay
  (bind _returnvalue (Actor|GetActorOfClass "/Game/Shared_Game_Mechanics/Cards/BP_Card_Dealer.BP_Card_Dealer_C"))
  (Variables|References|SetCard%20Dealer%20Reference _returnvalue)
  (bind _returnvalue_2 (Actor|GetActorOfClass "/Game/Shared_Game_Mechanics/Turn_Taking/BP_Turn_Manager.BP_Turn_Manager_C"))
  (Variables|References|SetTurn%20Manager%20Reference _returnvalue_2)
  (bind _outactors (Actor|GetAllActorsOfClasswithTag "/Game/Shared_Game_Mechanics/Cards/BP_CardPile.BP_CardPile_C" "I_Doubt_It_Card_Pile"))
  (Variables|Default|SetI%20Doubt%20It%20Card%20Pile (Utilities|Array|Get(acopy) _outactors)))

(fn ConstructionScript)

(fn SetupGame
  (bind _returnvalue (Actor|GetActorOfClass "/Game/Player/BP_Player.BP_Player_C"))
  (Utilities|Array|Add (Variables|Default|GetPlaying%20Characters) _returnvalue)
  (bind _outactors (Actor|GetAllActorsOfClasswithTag "/Game/NPCs/BP_NPC.BP_NPC_C" "I_Doubt_It_Participant"))
  (Utilities|Array|AppendArray (Variables|Default|GetPlaying%20Characters) _outactors)
  (Default|SetupCards (Variables|References|GetCard%20Dealer%20Reference) "NewEnumerator0")
  (Default|ShuffleCards (Variables|References|GetCard%20Dealer%20Reference))
  (Default|ClearCardPile (Variables|Default|GetI%20Doubt%20It%20Card%20Pile)))

(fn StartGame
  (Default|DealCards (Variables|References|GetCard%20Dealer%20Reference) "NewEnumerator0" (Variables|Default|GetPlaying%20Characters))
  (Default|SetupMainGame (Variables|References|GetTurn%20Manager%20Reference) "NewEnumerator0" (Variables|Default|GetPlaying%20Characters)))

(fn CheckifGameOver
  (bind _array_element (Utilities|Array|ForEachLoopwithBreak (Variables|Default|GetPlaying%20Characters))
    (:LoopBody
      (if (Utilities|Array|IsEmpty (Variables|/Game/Shared_Game_Mechanics/BPC_CurrentHand.BPC_CurrentHand_C|GetCurrent%20Hand (Actor|GetComponentbyClass _array_element "/Game/Shared_Game_Mechanics/BPC_CurrentHand.BPC_CurrentHand_C")))
        (LocalVariables|SetGame%20Over? true)))
    (:Completed
      (if (LocalVariables|GetGame%20Over?)
        (CallFunction|EndGame)
        (else
          (Default|NextPlayerTurn (Variables|References|GetTurn%20Manager%20Reference)))))))

(fn EndGame
  (Development|PrintString "I DOUBT IT GAME OVER"))

(fn EndPlayerTurn
  (params (Player :type Actor%20Object%20Reference) (Cards%20Played :type Array%20of%20BP%20Card%20Object%20References))
  (Variables|Default|SetMost%20Recent%20Played%20Cards Cards%20Played)
  (for _array_element Cards%20Played
    (Default|AddCardtoPile (Variables|References|GetCard%20Dealer%20Reference) _array_element (Variables|Default|GetI%20Doubt%20It%20Card%20Pile) true)
    (Default|RemoveCardfromPlayerHand (Variables|References|GetCard%20Dealer%20Reference) Player _array_element))
  (CallFunction|CheckifGameOver))

(fn DoubtCheck
  (params (Player%20Calling%20Doubt :type Actor%20Object%20Reference))
  (bind _current_card_value_to_be_played (Variables|Default|GetCurrent%20Card%20Value%20To%20Be%20Played))
  (bind _returnvalue (- _current_card_value_to_be_played 1))
  (for _array_element (Variables|Default|GetMost%20Recent%20Played%20Cards)
    (bind _card_info (Default|GetCardInfo _array_element))
    (if (not (== (.NumericalValue (Utilities|Struct|BreakStruct_Card _card_info)) (Math|Integer|SelectInt 13 _returnvalue (== _returnvalue -1))))
      (LocalVariables|SetDoubt%20Valid true)))
  (if (LocalVariables|GetDoubt%20Valid)
    (CallFunction|DoubtCorrect)
    (else
      (CallFunction|DoubtIncorrect Player%20Calling%20Doubt))))

(fn DoubtCorrect
  (bind _turn_manager_reference (Variables|References|GetTurn%20Manager%20Reference))
  (bind _playing_characters (Variables|/Game/Shared_Game_Mechanics/Turn_Taking/BP_Turn_Manager.BP_Turn_Manager_C|GetPlaying%20Characters _turn_manager_reference))
  (bind _current_character_turn_index_ (Variables|/Game/Shared_Game_Mechanics/Turn_Taking/BP_Turn_Manager.BP_Turn_Manager_C|GetCurrent%20Character%20Turn%20Index%20 _turn_manager_reference))
  (for _array_element (Variables|/Game/Shared_Game_Mechanics/Cards/BP_CardPile.BP_CardPile_C|GetCardsInPile (Variables|Default|GetI%20Doubt%20It%20Card%20Pile))
    (Default|RemoveCardfromPile (Variables|References|GetCard%20Dealer%20Reference) _array_element (Variables|Default|GetI%20Doubt%20It%20Card%20Pile))
    (Default|AddCardtoPlayerHand (Variables|References|GetCard%20Dealer%20Reference) (Utilities|Array|Get(acopy) _playing_characters (Math|Integer|SelectInt (- (Utilities|Array|Length _playing_characters) 1) _current_character_turn_index_ (== _current_character_turn_index_ 0))) _array_element)))

(fn DoubtIncorrect
  (params (Player%20Who%20Doubted :type Actor%20Object%20Reference))
  (for _array_element (Variables|/Game/Shared_Game_Mechanics/Cards/BP_CardPile.BP_CardPile_C|GetCardsInPile (Variables|Default|GetI%20Doubt%20It%20Card%20Pile))
    (Default|RemoveCardfromPile (Variables|References|GetCard%20Dealer%20Reference) _array_element (Variables|Default|GetI%20Doubt%20It%20Card%20Pile))
    (Default|AddCardtoPlayerHand (Variables|References|GetCard%20Dealer%20Reference) Player%20Who%20Doubted _array_element)))