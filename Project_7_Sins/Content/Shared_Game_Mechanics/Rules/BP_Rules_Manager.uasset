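; Rules manager that shows and hides the how-to-play widget for the bar's current card game: I Doubt It, Auction or Rat Screw.
; It creates all three widgets on BeginPlay and picks one by GM_Bar's CurrentPlayingGame.
; Showing pauses the game and enables UI input with the cursor.
; Hiding unpauses, plays the shrink, restores game input and removes the widget on a short timer, which reopening cancels.
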(event EventBeginPlay
  (bind _returnvalue (UserInterface|CreateWidget "/Game/UI/Non_Diegetic/Rules/WBP_Auction_Rules.WBP_Auction_Rules_C"))
  (Variables|Default|SetAuction%20Rules%20Ref _returnvalue)
  (bind _returnvalue_2 (UserInterface|CreateWidget "/Game/UI/Non_Diegetic/Rules/WBP_Rat_Screw_Rules.WBP_Rat_Screw_Rules_C"))
  (Variables|Default|SetRat%20Screw%20Rules%20Ref _returnvalue_2)
  (bind _returnvalue_3 (UserInterface|CreateWidget "/Game/UI/Non_Diegetic/Rules/WBP_I_Doubt_It_Rules.WBP_I_Doubt_It_Rules_C"))
  (Variables|Default|SetI%20Doubt%20It%20Rules%20Ref _returnvalue_3))

(fn ConstructionScript)

(fn ShowRules
  (Utilities|Time|ClearandInvalidateTimerbyHandle (Variables|Default|GetRemove%20from%20parent%20timer))
  (bind _asgm_bar (Utilities|Casting|CastToGM_Bar (Game|GetGameMode)))
  (Default|PausePlayingGame _asgm_bar)
  (Variables|Default|SetRules%20Shown true)
  (UserInterface|Viewport|AddtoViewport (Utilities|Select :Index (Variables|/Game/Modes_Instances/Modes/GM_Bar.GM_Bar_C|GetCurrent%20Playing%20Game _asgm_bar) :NewEnumerator0 (Variables|Default|GetI%20Doubt%20It%20Rules%20Ref) :NewEnumerator1 (Variables|Default|GetAuction%20Rules%20Ref) :NewEnumerator2 (Variables|Default|GetRat%20Screw%20Rules%20Ref) :NewEnumerator3 0 :NewEnumerator4 0 :NewEnumerator5 0) 0)
  (Input|SetInputModeGameandUI (Game|GetPlayerController 0) (Utilities|Select :Index (Variables|/Game/Modes_Instances/Modes/GM_Bar.GM_Bar_C|GetCurrent%20Playing%20Game _asgm_bar) :NewEnumerator0 (Variables|Default|GetI%20Doubt%20It%20Rules%20Ref) :NewEnumerator1 (Variables|Default|GetAuction%20Rules%20Ref) :NewEnumerator2 (Variables|Default|GetRat%20Screw%20Rules%20Ref) :NewEnumerator3 0 :NewEnumerator4 0 :NewEnumerator5 0) "DoNotLock" true false)
  (Variables|/Script/Engine.PlayerController|SetbShowMouseCursor (Game|GetPlayerController 0) true))

(fn HideRules
  (bind _asgm_bar (Utilities|Casting|CastToGM_Bar (Game|GetGameMode)))
  (Default|UnpausePlayingGame _asgm_bar)
  (Variables|Default|SetRules%20Shown false)
  (switch Utilities|FlowControl|Switch|SwitchonEnum_All_Game_Names (Variables|/Game/Modes_Instances/Modes/GM_Bar.GM_Bar_C|GetCurrent%20Playing%20Game _asgm_bar)
    (:NewEnumerator0
      (Default|ShrinkRules (Variables|Default|GetI%20Doubt%20It%20Rules%20Ref)))
    (:NewEnumerator1
      (Default|ShrinkRules (Variables|Default|GetAuction%20Rules%20Ref)))
    (:NewEnumerator2
      (Default|ShrinkRules (Variables|Default|GetRat%20Screw%20Rules%20Ref))))
  (bind _returnvalue (Utilities|Time|SetTimerbyFunctionName (Utilities|Select :Index (Variables|/Game/Modes_Instances/Modes/GM_Bar.GM_Bar_C|GetCurrent%20Playing%20Game _asgm_bar) :NewEnumerator0 (Variables|Default|GetI%20Doubt%20It%20Rules%20Ref) :NewEnumerator1 (Variables|Default|GetAuction%20Rules%20Ref) :NewEnumerator2 (Variables|Default|GetRat%20Screw%20Rules%20Ref) :NewEnumerator3 0 :NewEnumerator4 0 :NewEnumerator5 0) "Remove from Parent" 0.2))
  (Variables|Default|SetRemove%20from%20parent%20timer _returnvalue)
  (Input|SetInputModeGameOnly (Game|GetPlayerController 0) false)
  (Variables|/Script/Engine.PlayerController|SetbShowMouseCursor (Game|GetPlayerController 0) false))