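; Card pile actor for doubted cards in the IDI card game, which lays out a given set of cards along a spline.
; AddCardsToDoubtedSpline spaces the cards evenly from end to end of DoubtedCardsSpline in world space.
; Each card is rotated along the look-at direction from the BP_Player actor to its spot on the spline.
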(fn ConstructionScript
  (|CallParentFunction))

(fn AddCardstoDoubtedSpline
  (params (Cards :type Array%20of%20BP%20Card%20Object%20References))
  (bind _returnvalue (Actor|GetActorOfClass "/Game/Player/BP_Player.BP_Player_C"))
  (for (_array_element _array_index) Cards
    (Transformation|SetActorLocation _array_element (Spline|GetLocationatDistanceAlongSpline (Variables|Default|GetDoubted%20Cards%20Spline) (* (/ (Spline|GetSplineLength (Variables|Default|GetDoubted%20Cards%20Spline)) (- (Utilities|Array|Length Cards) 1)) _array_index) "World") false false)
    (Transformation|SetActorRotation _array_element (Math|Rotator|FindLookatRotation (Transformation|GetActorLocation _returnvalue) (Spline|GetLocationatDistanceAlongSpline (Variables|Default|GetDoubted%20Cards%20Spline) (* (/ (Spline|GetSplineLength (Variables|Default|GetDoubted%20Cards%20Spline)) (- (Utilities|Array|Length Cards) 1)) _array_index) "World")))))