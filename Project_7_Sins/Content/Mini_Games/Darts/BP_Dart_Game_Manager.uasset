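; Manager for the 301/501 darts mini-game between the player and a tagged NPC opponent.
; Timers called by function name chain setup, turns and character swaps between throwing and waiting spots, with camera fades.
; Normalized aim values map onto board extents, and the nearest score-point actor to the hit gives the score.
; It handles busts, wins and scoreboard updates, and can convert score points back into randomly offset aim values.
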(event EventBeginPlay
  (Utilities|SetupReferences
    (:Done
      (Utilities|SetupDartActors))))

(fn ConstructionScript)

(fn SetupGame
  (bind _returnvalue (Math|Random|RandomBoolwithWeight 0.0))
  (Default|HideStartingUI (Variables|References|GetDart%20Board%20Ref))
  (Main|SetupDifficulty)
  (Main|SetupGameMode)
  (Development|PrintString "DARTS SETUP")
  (Variables|Checks|SetPlayer%20Started%20First _returnvalue)
  (Variables|Round|SetActive%20Player (select _returnvalue (Variables|References|GetPlayer%20Ref) (Variables|References|GetDart%20NPC%20Opponent)))
  (CameraFades|CameraFadeOut (Variables|FadeTimings|GetFade%20Time%20For%20Setup))
  (Utilities|Time|SetTimerbyFunctionName 0 "Move Characters" (Variables|FadeTimings|GetFade%20Time%20For%20Setup))
  (Utilities|Time|SetTimerbyFunctionName 0 "Begin Game" (* (Variables|FadeTimings|GetFade%20Time%20For%20Setup) 2.0)))

(fn SetupDifficulty
  (Utilities|Map|Add (Variables|/Game/NPCs/BP_NPC.BP_NPC_C|GetGame%20->%20Difficulty (Variables|References|GetDart%20NPC%20Opponent)) "NewEnumerator4" (Variables|/Game/Mini_Games/Darts/BP_Dart_Board.BP_Dart_Board_C|GetSelected%20Difficulty (Variables|References|GetDart%20Board%20Ref))))

(fn SetupGameMode
  (bind _returnvalue (Class|KismetSystemLibrary|MakeLiteralInteger 301))
  (bind _returnvalue_2 (Class|KismetSystemLibrary|MakeLiteralInteger 501))
  (bind _dart_board_ref (Variables|References|GetDart%20Board%20Ref))
  (bind _dart_npc_opponent (Variables|References|GetDart%20NPC%20Opponent))
  (bind _selected_dart_mode (Variables|/Game/Mini_Games/Darts/BP_Dart_Board.BP_Dart_Board_C|GetSelected%20Dart%20Mode _dart_board_ref))
  (bind _npc_name (Variables|/Game/NPCs/BP_NPC.BP_NPC_C|GetNPC%20Name _dart_npc_opponent))
  (bind _returnvalue_3 (Utilities|String|EnumtoString _npc_name))
  (bind _returnvalue_4 (Utilities|Select :Index _selected_dart_mode :NewEnumerator0 _returnvalue_2 :NewEnumerator1 _returnvalue))
  (bind _returnvalue_5 (Utilities|String|StringToName _returnvalue_3))
  (Utilities|Map|Add (Variables|Round|GetPlayer%20->%20Score) (Variables|References|GetPlayer%20Ref) _returnvalue_4)
  (Utilities|Map|Add (Variables|Round|GetPlayer%20->%20Score) (Variables|References|GetDart%20NPC%20Opponent) _returnvalue_4)
  (Default|Setup (Variables|/Game/Mini_Games/Darts/BP_Dart_Board.BP_Dart_Board_C|GetScoreboard%20Widget%20Ref (Variables|References|GetDart%20Board%20Ref)) (select (== (Variables|Round|GetActive%20Player) (Variables|References|GetPlayer%20Ref)) (Utilities|Array|MakeArray "Soul" _returnvalue_5) (Utilities|Array|MakeArray _returnvalue_5 "Soul")) (Variables|/Game/Mini_Games/Darts/BP_Dart_Board.BP_Dart_Board_C|GetSelected%20Dart%20Mode (Variables|References|GetDart%20Board%20Ref))))

(fn BeginGame
  (Variables|Checks|SetDarts%20Game%20Active true)
  (Development|PrintString "DARTS GAME BEGUN")
  (Main|PlayerTurn)
  (Default|ShowScoreboard (Variables|References|GetDart%20Board%20Ref)))

(fn PlayerTurn
  (Utilities|Time|SetTimerbyFunctionName (Variables|Round|GetActive%20Player) "Take Turn" (Variables|PlayerSpecific|GetPlayer%20Stop%20Bar%20Delay))
  (if (== (Variables|Round|GetActive%20Player) (Variables|References|GetPlayer%20Ref))
    (Default|StartSliders (Variables|References|GetDart%20Board%20Ref))))

(fn PlayDart
  (bind _dart_board_ref (Variables|References|GetDart%20Board%20Ref))
  (bind _active_player (Variables|Round|GetActive%20Player))
  (bind _player_ref (Variables|References|GetPlayer%20Ref))
  (bind _dart_board_ref_2 (Variables|References|GetDart%20Board%20Ref))
  (bind _player_started_first (Variables|Checks|GetPlayer%20Started%20First))
  (bind _active_player_2 (Variables|Round|GetActive%20Player))
  (bind _player_ref_2 (Variables|References|GetPlayer%20Ref))
  (bind _active_player_3 (Variables|Round|GetActive%20Player))
  (bind _returnvalue (== _active_player_2 _player_ref_2))
  (bind _returnvalue_2 (== _active_player _player_ref))
  (bind _dart_board_extent_sw (Variables|/Game/Mini_Games/Darts/BP_Dart_Board.BP_Dart_Board_C|GetDart%20Board%20Extent%20SW _dart_board_ref))
  (bind _current_player_aim_values (Variables|/Game/Mini_Games/Darts/BP_Dart_Board.BP_Dart_Board_C|GetCurrent%20Player%20Aim%20Values _dart_board_ref_2))
  (bind _returnvalue_3 (Transformation|GetWorldLocation _dart_board_extent_sw))
  (bind _returnvalue_4 (Math|Integer|SelectInt 0 1 _returnvalue))
  (bind _returnvalue_5 (Math|Integer|SelectInt 1 0 _returnvalue))
  (bind _output (Utilities|Array|Get(acopy) _current_player_aim_values 1))
  (bind _output_2 (Utilities|Array|Get(acopy) _current_player_aim_values))
  (bind _returnvalue_6 (Math|Integer|SelectInt _returnvalue_4 _returnvalue_5 _player_started_first))
  (Variables|/Game/Player/BP_Player.BP_Player_C|SetMy%20Turn (Variables|References|GetPlayer%20Ref) false)
  (Development|PrintString "PLAY DART")
  (Development|PrintString (Utilities|String|Append (Utilities|String|ToString(Float) _output_2) (Utilities|String|ToString(Float) _output)))
  (bind _output_get (LocalVariables|SetDart%20Hit%20Loc (Math|Vector|MakeVector (.X (Math|Vector|BreakVector (Transformation|GetWorldLocation (Variables|/Game/Mini_Games/Darts/BP_Dart_Board.BP_Dart_Board_C|GetDart%20Board%20X%20Location (Variables|References|GetDart%20Board%20Ref))))) (.y (+ _returnvalue_3 (Math|Vector|MakeVector 0.0 (* (Math|Vector|Distance(Vector) _returnvalue_3 (Transformation|GetWorldLocation (Variables|/Game/Mini_Games/Darts/BP_Dart_Board.BP_Dart_Board_C|GetDart%20Board%20Extent%20SE _dart_board_ref))) _output_2) 0.0))) (.z (+ _returnvalue_3 (Math|Vector|MakeVector 0.0 0.0 (* (Math|Vector|Distance(Vector) _returnvalue_3 (Transformation|GetWorldLocation (Variables|/Game/Mini_Games/Darts/BP_Dart_Board.BP_Dart_Board_C|GetDart%20Board%20Extent%20NW _dart_board_ref))) _output)))))))
  (Rendering|Debug|DrawDebugSphere _output_get 0.01 12 "(R=1.000000,G=1.000000,B=1.000000,A=1.000000)" 1e+02 0.05)
  (Default|ActivateDart (Utilities|Array|Get(acopy) (Variables|References|GetDarts) (- (Variables|Round|GetDarts%20Available) 1)) (+ (* (Transformation|GetActorForwardVector _active_player_3) 1e+02) (Transformation|GetActorLocation _active_player_3)) (LocalVariables|GetDart%20Hit%20Loc))
  ;[0 0 0] Calculate score from aim values
  (bind _asbp_dart_score_point (Utilities|Casting|CastToBP_Dart_Score_Point (.ReturnValue (Actor|FindNearestActor (LocalVariables|GetDart%20Hit%20Loc) (Variables|/Game/Mini_Games/Darts/BP_Dart_Board.BP_Dart_Board_C|GetScore%20Point%20Actors (Variables|References|GetDart%20Board%20Ref))))))
  (bind _score_value (Default|GetScore _asbp_dart_score_point))
  (Development|PrintString (Utilities|String|ToString(Integer) _score_value))
  (Utilities|Array|Add (Variables|Round|GetCurrent%20Round%20Scores) _score_value)
  (Default|ResetCurrentPlayerAimValues (Variables|References|GetDart%20Board%20Ref))
  (bind _game_over (Main|CheckifGameOver _score_value))
  (if _game_over
    (Default|ChangeDartScore (Variables|/Game/Mini_Games/Darts/BP_Dart_Board.BP_Dart_Board_C|GetScoreboard%20Widget%20Ref (Variables|References|GetDart%20Board%20Ref)) (- 4 (Variables|Round|GetDarts%20Available)) _score_value (Math|Integer|SelectInt (Math|Integer|SelectInt 0 1 _returnvalue_2) (Math|Integer|SelectInt 1 0 _returnvalue_2) (Variables|Checks|GetPlayer%20Started%20First)) false)
    (Main|GameOver)
    (else
      (bind _busted (Main|BustCheck _score_value))
      (if _busted
        (Default|ChangeDartScore (Variables|/Game/Mini_Games/Darts/BP_Dart_Board.BP_Dart_Board_C|GetScoreboard%20Widget%20Ref (Variables|References|GetDart%20Board%20Ref)) (- 4 (Variables|Round|GetDarts%20Available)) 0 _returnvalue_6 true)
        (Development|PrintString "BUST")
        (Utilities|Time|SetTimerbyFunctionName 0 "End Player Turn" (Variables|Round|GetPlayer%20Turn%20Interval))
        (else
          (Default|ChangeDartScore (Variables|/Game/Mini_Games/Darts/BP_Dart_Board.BP_Dart_Board_C|GetScoreboard%20Widget%20Ref (Variables|References|GetDart%20Board%20Ref)) (- 4 (Variables|Round|GetDarts%20Available)) _score_value _returnvalue_6 false)
          (bind _result (Math|Integer|DecrementInt (Variables|Round|GetDarts%20Available))
            (:%20%20
              (if (<= _result 0)
                (Utilities|Time|SetTimerbyFunctionName 0 "End Player Turn" (Variables|Round|GetPlayer%20Turn%20Interval))
                (else
                  (Utilities|Time|SetTimerbyFunctionName 0 "Player Turn" (Variables|Round|GetPlayer%20Turn%20Interval)))))))))))

(fn EndPlayerTurn
  (Variables|Round|SetDarts%20Available 3)
  (for _array_element (Variables|References|GetDarts)
    (Default|DeactivateDart _array_element))
  (for _array_element_2 (Variables|Round|GetCurrent%20Round%20Scores)
    (LocalVariables|SetTotal%20Player%20Score%20for%20Round (+ (LocalVariables|GetTotal%20Player%20Score%20for%20Round) _array_element_2)))
  (Utilities|Array|Clear (Variables|Round|GetCurrent%20Round%20Scores))
  (Utilities|Map|Add (Variables|Round|GetPlayer%20->%20Score) (Variables|Round|GetActive%20Player) (- (.Value (Utilities|Map|Find (Variables|Round|GetPlayer%20->%20Score) (Variables|Round|GetActive%20Player))) (LocalVariables|GetTotal%20Player%20Score%20for%20Round)))
  (Default|UpdatePlayerScore (Variables|/Game/Mini_Games/Darts/BP_Dart_Board.BP_Dart_Board_C|GetScoreboard%20Widget%20Ref (Variables|References|GetDart%20Board%20Ref)) (Math|Integer|SelectInt (Math|Integer|SelectInt 0 1 (== (Variables|Round|GetActive%20Player) (Variables|References|GetPlayer%20Ref))) (Math|Integer|SelectInt 1 0 (== (Variables|Round|GetActive%20Player) (Variables|References|GetPlayer%20Ref))) (Variables|Checks|GetPlayer%20Started%20First)) (.Value (Utilities|Map|Find (Variables|Round|GetPlayer%20->%20Score) (Variables|Round|GetActive%20Player))))
  (if (== (Variables|Round|GetActive%20Player) (Variables|References|GetPlayer%20Ref))
    (Variables|/Game/Player/BP_Player.BP_Player_C|SetMy%20Turn (Variables|References|GetPlayer%20Ref) false)
    (Variables|Round|SetActive%20Player (Variables|References|GetDart%20NPC%20Opponent))
    (Default|HideBothSliders (Variables|References|GetDart%20Board%20Ref))
    (else
      (Variables|Round|SetActive%20Player (Variables|References|GetPlayer%20Ref))))
  (Main|MoveCharacters)
  (Utilities|Time|SetTimerbyFunctionName 0 "Player Turn" (Variables|Round|GetPlayer%20Turn%20Interval)))

(fn CheckifGameOver
  (params (Score :type Integer))
  (return (== (- (.Value (Utilities|Map|Find (Variables|Round|GetPlayer%20->%20Score) (Variables|Round|GetActive%20Player))) Score) 0)))

(fn MoveCharacters
  (bind _dart_board_ref (Variables|References|GetDart%20Board%20Ref))
  (bind _dart_board_ref_2 (Variables|References|GetDart%20Board%20Ref))
  (bind _dart_board_ref_3 (Variables|References|GetDart%20Board%20Ref))
  (bind _dart_playing_position (Variables|/Game/Mini_Games/Darts/BP_Dart_Board.BP_Dart_Board_C|GetDart%20Playing%20Position _dart_board_ref_2))
  (bind _dart_non_playing_position (Variables|/Game/Mini_Games/Darts/BP_Dart_Board.BP_Dart_Board_C|GetDart%20Non-Playing%20Position _dart_board_ref_3))
  (bind _dart_playing_position_2 (Variables|/Game/Mini_Games/Darts/BP_Dart_Board.BP_Dart_Board_C|GetDart%20Playing%20Position _dart_board_ref))
  (bind _returnvalue (Transformation|GetWorldRotation _dart_non_playing_position))
  (bind _returnvalue_2 (Transformation|GetWorldLocation _dart_playing_position_2))
  (bind _returnvalue_3 (Transformation|GetWorldLocation _dart_playing_position))
  (bind _returnvalue_4 (Transformation|GetWorldLocation _dart_non_playing_position))
  (bind (_x _y) (Math|Vector|BreakVector _returnvalue_4))
  (bind (_x_2 _y_2) (Math|Vector|BreakVector _returnvalue_4))
  (bind (_x_3 _y_3) (Math|Vector|BreakVector _returnvalue_2))
  (bind (_x_4 _y_4) (Math|Vector|BreakVector _returnvalue_3))
  (if (== (Variables|Round|GetActive%20Player) (Variables|References|GetPlayer%20Ref))
    (Transformation|SetActorLocation (Variables|References|GetPlayer%20Ref) (Math|Vector|MakeVector _x_4 _y_4 (.Z (Math|Vector|BreakVector (Transformation|GetActorLocation (Variables|References|GetPlayer%20Ref))))) false false)
    (Pawn|SetControlRotation (Pawn|GetController (Variables|References|GetPlayer%20Ref)) (Transformation|GetWorldRotation _dart_playing_position))
    (Transformation|SetActorLocation (Variables|References|GetDart%20NPC%20Opponent) (Math|Vector|MakeVector _x _y (.Z (Math|Vector|BreakVector (Transformation|GetActorLocation (Variables|References|GetDart%20NPC%20Opponent))))) false false)
    (Transformation|SetActorRotation (Variables|References|GetDart%20NPC%20Opponent) _returnvalue)
    (else
      (Transformation|SetActorLocation (Variables|References|GetDart%20NPC%20Opponent) (Math|Vector|MakeVector _x_3 _y_3 (.Z (Math|Vector|BreakVector (Transformation|GetActorLocation (Variables|References|GetDart%20NPC%20Opponent))))) false false)
      (Transformation|SetActorRotation (Variables|References|GetDart%20NPC%20Opponent) (Transformation|GetWorldRotation _dart_playing_position_2))
      (Transformation|SetActorLocation (Variables|References|GetPlayer%20Ref) (Math|Vector|MakeVector _x_2 _y_2 (.Z (Math|Vector|BreakVector (Transformation|GetActorLocation (Variables|References|GetPlayer%20Ref))))) false false)
      (Pawn|SetControlRotation (Pawn|GetController (Variables|References|GetPlayer%20Ref)) _returnvalue)))
  (CameraFades|CameraFadein (Math|Float|SelectFloat (Variables|FadeTimings|GetFade%20Time%20For%20Setup) (Variables|FadeTimings|GetFade%20Time%20For%20Moving) (== (Variables|Round|GetCurrent%20Round%20Index) 0))))

(fn CameraFadein
  (params (Duration :type Float%20%28double-precision%29))
  (CameraFades|StartCameraFade :self (Game|GetPlayerCameraManager 0) :FromAlpha 1.0 :Duration Duration))

(fn CameraFadeOut
  (params (Duration :type Float%20%28double-precision%29))
  (CameraFades|StartCameraFade :self (Game|GetPlayerCameraManager 0) :ToAlpha 1.0 :Duration Duration :bHoldWhenFinished true))

(fn Cancel/LeaveGame
  (Input|SetIgnoreMoveInput (Pawn|GetController (Variables|References|GetPlayer%20Ref)) false)
  (Variables|Checks|SetDarts%20Game%20Active false)
  (Default|DEBUGLeaveCurrentGame (Variables|References|GetAs%20GM%20Bar))
  (Default|HideScoreboard (Variables|References|GetDart%20Board%20Ref)))

(fn StopPlayerAimBar
  (Default|StopPlayerAimBar (Variables|References|GetDart%20Board%20Ref))
  (if (== (Utilities|Array|Length (Variables|/Game/Mini_Games/Darts/BP_Dart_Board.BP_Dart_Board_C|GetCurrent%20Player%20Aim%20Values (Variables|References|GetDart%20Board%20Ref))) 1)
    (Variables|/Game/Player/BP_Player.BP_Player_C|SetMy%20Turn (Variables|References|GetPlayer%20Ref) false)
    (Utilities|Time|SetTimerbyFunctionName (Variables|References|GetPlayer%20Ref) "Take Turn" (Variables|PlayerSpecific|GetPlayer%20Stop%20Bar%20Delay))))

(fn GameOver
  (Development|PrintString "DARTS GAME OVER")
  (Development|PrintString (Utilities|String|Append "DARTS WINNER IS : " (Utilities|GetDisplayName (Variables|Round|GetActive%20Player))))
  (Default|ShowWinningText (Variables|References|GetDart%20Board%20Ref) (== (Variables|Round|GetActive%20Player) (Variables|References|GetPlayer%20Ref)) (Variables|/Game/NPCs/BP_NPC.BP_NPC_C|GetNPC%20Name (Variables|References|GetDart%20NPC%20Opponent))))

(fn BustCheck
  (params (Dart%20Score :type Integer))
  (return (< (- (.Value (Utilities|Map|Find (Variables|Round|GetPlayer%20->%20Score) (Variables|Round|GetActive%20Player))) Dart%20Score) 0)))

(fn CalculateAimValuesfromScorePointActor
  (params (Score%20Point%20Actor :type BP%20Dart%20Score%20Point%20Object%20Reference))
  (bind _returnvalue (Transformation|GetActorLocation Score%20Point%20Actor))
  (bind _dart_board_ref (Variables|References|GetDart%20Board%20Ref))
  (bind (_x _y _z) (Math|Vector|BreakVector _returnvalue))
  (bind _dart_board_extent_sw (Variables|/Game/Mini_Games/Darts/BP_Dart_Board.BP_Dart_Board_C|GetDart%20Board%20Extent%20SW _dart_board_ref))
  (bind _returnvalue_2 (Transformation|GetWorldLocation _dart_board_extent_sw))
  (bind (_x_2 _y_2 _z_2) (Math|Vector|BreakVector _returnvalue_2))
  (bind _score_value (Default|GetScore Score%20Point%20Actor))
  (LocalVariables|SetRandom%20Deviation%20To%20Use (Math|Float|SelectFloat (LocalVariables|GetRandom%20Deviation%20Treble) (Math|Float|SelectFloat (LocalVariables|GetRandom%20Deviation%20Double) (Math|Float|SelectFloat (LocalVariables|GetRandom%20Deviation%20Miss) (Math|Float|SelectFloat (LocalVariables|GetRandom%20Deviation%20Green) (Math|Float|SelectFloat (LocalVariables|GetRandom%20Deviation%20Bullseye) (LocalVariables|GetRandom%20Deviation%20Normal) (== _score_value 50)) (== _score_value 25)) (== _score_value 0)) (Variables|/Game/Mini_Games/Darts/BP_Dart_Score_Point.BP_Dart_Score_Point_C|GetDouble? Score%20Point%20Actor)) (Variables|/Game/Mini_Games/Darts/BP_Dart_Score_Point.BP_Dart_Score_Point_C|GetTreble? Score%20Point%20Actor)))
  (return (Utilities|Array|MakeArray (+ (/ (- _y _y_2) (Math|Vector|Distance(Vector) _returnvalue_2 (Transformation|GetWorldLocation (Variables|/Game/Mini_Games/Darts/BP_Dart_Board.BP_Dart_Board_C|GetDart%20Board%20Extent%20SE _dart_board_ref)))) (Math|Random|RandomFloatinRange (* (LocalVariables|GetRandom%20Deviation%20Normal) -1.0) (LocalVariables|GetRandom%20Deviation%20Normal))) (+ (/ (- _z _z_2) (Math|Vector|Distance(Vector) _returnvalue_2 (Transformation|GetWorldLocation (Variables|/Game/Mini_Games/Darts/BP_Dart_Board.BP_Dart_Board_C|GetDart%20Board%20Extent%20NW _dart_board_ref)))) (Math|Random|RandomFloatinRange (* (LocalVariables|GetRandom%20Deviation%20Normal) -1.0) (LocalVariables|GetRandom%20Deviation%20Normal))))))