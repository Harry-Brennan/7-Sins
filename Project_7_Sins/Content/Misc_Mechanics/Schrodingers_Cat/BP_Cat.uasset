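; BP_Cat is a Schrödinger's cat actor that relocates after the player has looked at it and then looks away.
; Once activated, a looping timer box-traces along the player's view to detect BPI_Cat actors and flag the cat as seen.
; Losing sight stops tracing, moves the cat using random PossiblePoints other than the current one, and re-arms tracing after a delay.
; Debug prints and trace drawing remain enabled.
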(event EventBeginPlay
  (bind _returnvalue (Actor|GetActorOfClass "/Game/Player/BP_Player.BP_Player_C"))
  (Variables|Default|SetPlayer%20Ref _returnvalue))

(fn ConstructionScript)

(fn ActivateCatTrace
  (Development|PrintString "ACTIVATE CAT TRACE")
  (bind _returnvalue (Utilities|Time|SetTimerbyFunctionName 0 "Cat Trace" 0.05 true))
  (Variables|Default|SetCat%20Trace%20Timer _returnvalue)
  (Variables|Default|SetTrace%20Active true))

(fn DeactivateCatTrace
  (Development|PrintString "DEACTIVATE CAT TRACE")
  (Utilities|Time|ClearandInvalidateTimerbyHandle (Variables|Default|GetCat%20Trace%20Timer))
  (Variables|Default|SetTrace%20Active false))

(fn CatTrace
  (bind _player_ref (Variables|Default|GetPlayer%20Ref))
  (bind _player_ref_2 (Variables|Default|GetPlayer%20Ref))
  (bind _outlocation (Actor|GetActorEyesViewPoint _player_ref_2))
  (bind _returnvalue (Pawn|GetControlRotation _player_ref :!class /Script/Engine.Pawn))
  (bind (_outhit _returnvalue_2) (Collision|BoxTraceByChannel _outlocation (+ (* (Math|Vector|GetForwardVector _returnvalue) 5e+03) _outlocation) "0.000000,128.000000,64.000000" _returnvalue "TraceTypeQuery2" false 0 "ForOneFrame"))
  (if _returnvalue_2
    (if (Utilities|DoesObjectImplementInterface (.HitActor (Collision|BreakHitResult _outhit)) "/Game/Misc_Mechanics/Schrodingers_Cat/BPI_Cat.BPI_Cat_C")
      (Variables|Default|SetActive true :!label _label)
      (elif (.bBlockingHit (Collision|BreakHitResult _outhit))
        (if (Variables|Default|GetActive)
          (Variables|Default|SetActive false :!label _label_2)
          (CallFunction|MoveCat)
          (CallFunction|DeactivateCatTrace))
        (else
          (goto _label))))
    (elif (Variables|Default|GetActive)
      (goto _label_2))))

(fn MoveCat
  (Development|PrintString "MOVE CAT")
  (bind _output_get (LocalVariables|SetAvailable%20Points (Variables|Default|GetPossible%20Points)))
  (Utilities|Array|RemoveItem _output_get (Variables|Default|GetCurrent%20Target%20Point))
  (Development|PrintString (Utilities|GetDisplayName (Variables|Default|GetCurrent%20Target%20Point)) true true "(R=0.066611,G=0.000000,B=1.000000,A=1.000000)" 1e+02)
  (bind _output_get_2 (Variables|Default|SetCurrent%20Target%20Point (.OutItem (Utilities|Array|Random (LocalVariables|GetAvailable%20Points)))))
  (Development|PrintString (Utilities|GetDisplayName _output_get_2) true true "(R=1.000000,G=0.000000,B=0.136464,A=1.000000)" 1e+02)
  (Transformation|SetActorLocationAndRotation (Transformation|GetActorLocation (.OutItem (Utilities|Array|Random (LocalVariables|GetAvailable%20Points)))) (Transformation|GetActorRotation (.OutItem (Utilities|Array|Random (LocalVariables|GetAvailable%20Points)))))
  (Utilities|Time|SetTimerbyFunctionName 0 "Activate Cat Trace" 1.0))