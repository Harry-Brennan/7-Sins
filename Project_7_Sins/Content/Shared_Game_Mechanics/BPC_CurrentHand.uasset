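; Component that manages a player's or NPC opponent's hand of cards across the shared card games.
; Hover cycles through the hand and toggles selection, with limits set by the current game and Auction round state and card actors giving visual feedback.
; The hand sorts by suit buckets, bubble-sorts by value or shuffles.
; Cards spread evenly along a spline, attached to camera or owner capsule, then non-NPC owners auto-hover the first.
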(fn SelectCard
  ;[0 0 0] Add the current hovered card to the selected cards array if it is not already selected and call corresponding function in card actor. If it is already selected then unselect it
  (if (Utilities|Array|ContainsItem (Variables|Default|GetSelected%20Cards) (Variables|Default|GetHovered%20Card))
    (Selection|DeselectCard)
    (else
      (bind _can_select_ (Selection|CanSelectCard (Variables|Default|GetHovered%20Card)))
      (if _can_select_
        (Utilities|Array|Add (Variables|Default|GetSelected%20Cards) (Variables|Default|GetHovered%20Card))
        (Default|SelectCardWhilstHeld (Variables|Default|GetHovered%20Card))
        (else
          (Default|ShakeCard (Variables|Default|GetHovered%20Card)))))))

(fn DeselectCard
  (bind _hovered_card (Variables|Default|GetHovered%20Card))
  ;[0 0 0] Remove hovered card from selected cards array and call corresponding function in card actor
  (Utilities|Array|RemoveItem (Variables|Default|GetSelected%20Cards) _hovered_card)
  (Default|UnSelectCardWhilstHeld _hovered_card))

(fn NextCard
  (bind _current_hand (Variables|Default|GetCurrent%20Hand))
  ;[0 0 0] Hover the next card in the array and unhover the current hovered card if it is not selected
  (bind _hovered_card (Variables|Default|GetHovered%20Card)
    (:then
      (if (Utilities|Array|ContainsItem (Variables|Default|GetSelected%20Cards) _hovered_card)
        _
        (else
          (Default|UnHoverCardWhilstHeld _hovered_card))))
    (:else
      _))
  (bind _output_get (Variables|Default|SetHovered%20Card (select (> (+ (Utilities|Array|FindItem (Variables|Default|GetCurrent%20Hand) (Variables|Default|GetHovered%20Card)) 1) (Utilities|Array|LastIndex (Variables|Default|GetCurrent%20Hand))) (Utilities|Array|Get(acopy) _current_hand) (Utilities|Array|Get(acopy) _current_hand (+ (Utilities|Array|FindItem (Variables|Default|GetCurrent%20Hand) (Variables|Default|GetHovered%20Card)) 1)))))
  (if (Utilities|Array|ContainsItem (Variables|Default|GetSelected%20Cards) _output_get)
    (Default|ShakeCard _output_get)
    (else
      (Default|HoverCardWhilstHeld _output_get))))

(fn PreviousCard
  (bind _current_hand (Variables|Default|GetCurrent%20Hand))
  ;[0 0 0] Same as next card but for the previous card in the array
  (bind _hovered_card (Variables|Default|GetHovered%20Card)
    (:then
      (if (Utilities|Array|ContainsItem (Variables|Default|GetSelected%20Cards) _hovered_card)
        _
        (else
          (Default|UnHoverCardWhilstHeld _hovered_card))))
    (:else
      _))
  (bind _output_get (Variables|Default|SetHovered%20Card (select (< (- (Utilities|Array|FindItem (Variables|Default|GetCurrent%20Hand) (Variables|Default|GetHovered%20Card)) 1) 0) (Utilities|Array|Get(acopy) _current_hand (Utilities|Array|LastIndex _current_hand)) (Utilities|Array|Get(acopy) _current_hand (- (Utilities|Array|FindItem (Variables|Default|GetCurrent%20Hand) (Variables|Default|GetHovered%20Card)) 1)))))
  (if (Utilities|Array|ContainsItem (Variables|Default|GetSelected%20Cards) _output_get)
    (Default|ShakeCard _output_get)
    (else
      (Default|HoverCardWhilstHeld _output_get))))

(fn ClearSelectedCards
  ;[0 0 0] Clears the selected cards
  (Utilities|Array|Clear (Variables|Default|GetSelected%20Cards)))

(fn HoverCheck
  (params (Card :type BP%20Card%20Object%20Reference))
  ;[0 0 0] Makes the passed card the hovered card and then checks if it is a selected card to then do either shake or hover
  (bind _output_get (Variables|Default|SetHovered%20Card Card))
  (if (Utilities|Array|ContainsItem (Variables|Default|GetSelected%20Cards) _output_get)
    (Default|ShakeCard _output_get)
    (else
      (Default|HoverCardWhilstHeld _output_get))))

(fn IsCardSelected?
  (params (Card :type BP%20Card%20Object%20Reference))
  ;[0 0 0] Checks if passed card is a selected card
  (return (Utilities|Array|ContainsItem (Variables|Default|GetSelected%20Cards) Card)))

(fn SortCurrentHand
  (params (Sort%20Method :type Enum_Card_Sort_Methods%20Enum :default "NewEnumerator0"))
  (Development|PrintString (Utilities|String|Append "SORTING : " (Utilities|String|EnumtoString Sort%20Method)))
  (switch Utilities|FlowControl|Switch|SwitchonEnum_Card_Sort_Methods Sort%20Method
    (:NewEnumerator0
      ;[0 0 0] Loop through current hand adding to the corresponding array of the suit of the current card in the loop
      (for _array_element (Variables|Default|GetCurrent%20Hand)
        (bind _card_info (Default|GetCardInfo _array_element))
        (Utilities|Array|Add (Utilities|Select :Index (.Suit (Utilities|Struct|BreakStruct_Card _card_info)) :NewEnumerator0 (LocalVariables|GetSpades) :NewEnumerator1 (LocalVariables|GetHearts) :NewEnumerator2 (LocalVariables|GetDiamonds) :NewEnumerator3 (LocalVariables|GetClubs) :NewEnumerator4 (LocalVariables|GetUnique)) _array_element))
      ;[0 0 0] Clear the current hand and then append the arrays so that the current hand is the suits in order
      (Utilities|Array|Clear (Variables|Default|GetCurrent%20Hand))
      (Utilities|Array|AppendArray (Variables|Default|GetCurrent%20Hand) (LocalVariables|GetSpades))
      (Utilities|Array|AppendArray (Variables|Default|GetCurrent%20Hand) (LocalVariables|GetHearts))
      (Utilities|Array|AppendArray (Variables|Default|GetCurrent%20Hand) (LocalVariables|GetDiamonds))
      (Utilities|Array|AppendArray (Variables|Default|GetCurrent%20Hand) (LocalVariables|GetClubs))
      (Utilities|Array|AppendArray (Variables|Default|GetCurrent%20Hand) (LocalVariables|GetUnique))
      (return))
    (:NewEnumerator1
      ;[0 0 0] Bubble sort ascending
      (bind _index (Utilities|FlowControl|ForLoopwithBreak 0 (- (Utilities|Array|Length (Variables|Default|GetCurrent%20Hand)) 1) :!label _label)
        (:LoopBody
          (LocalVariables|SetSwapped false)
          (for _index_2 (range 0 (- (- (Utilities|Array|Length (Variables|Default|GetCurrent%20Hand)) _index) 1))
            (bind _card_info_2 (Default|GetCardInfo (Utilities|Array|Get(acopy) (Variables|Default|GetCurrent%20Hand) _index_2)))
            (Utilities|IsValid (Utilities|Array|Get(acopy) (Variables|Default|GetCurrent%20Hand) (+ _index_2 1))
              (:Is%20Valid
                (bind _card_info_3 (Default|GetCardInfo (Utilities|Array|Get(acopy) (Variables|Default|GetCurrent%20Hand) (+ _index_2 1))))
                (if (> (Utilities|Struct|BreakStruct_Card _card_info_2) (Utilities|Struct|BreakStruct_Card _card_info_3))
                  (LocalVariables|SetSwapped true)
                  (LocalVariables|SetTemp%20Card (Utilities|Array|Get(acopy) (Variables|Default|GetCurrent%20Hand) _index_2))
                  (Utilities|Array|SetArrayElem (Variables|Default|GetCurrent%20Hand) _index_2 (Utilities|Array|Get(acopy) (Variables|Default|GetCurrent%20Hand) (+ _index_2 1)))
                  (Utilities|Array|SetArrayElem (Variables|Default|GetCurrent%20Hand) (+ _index_2 1) (LocalVariables|GetTemp%20Card))))))
          (if (not (LocalVariables|GetSwapped))
            (goto _label Break)))
        (:Completed
          (return))))
    (:NewEnumerator4
      ;[0 0 0] Bubble sort descending
      (bind _index_3 (Utilities|FlowControl|ForLoopwithBreak 0 (- (Utilities|Array|Length (Variables|Default|GetCurrent%20Hand)) 1) :!label _label_2)
        (:LoopBody
          (LocalVariables|SetSwapped false)
          (for _index_4 (range 0 (- (- (Utilities|Array|Length (Variables|Default|GetCurrent%20Hand)) _index_3) 1))
            (bind _card_info_4 (Default|GetCardInfo (Utilities|Array|Get(acopy) (Variables|Default|GetCurrent%20Hand) _index_4)))
            (Utilities|IsValid (Utilities|Array|Get(acopy) (Variables|Default|GetCurrent%20Hand) (+ _index_4 1))
              (:Is%20Valid
                (bind _card_info_5 (Default|GetCardInfo (Utilities|Array|Get(acopy) (Variables|Default|GetCurrent%20Hand) (+ _index_4 1))))
                (if (< (Utilities|Struct|BreakStruct_Card _card_info_4) (Utilities|Struct|BreakStruct_Card _card_info_5))
                  (LocalVariables|SetSwapped true)
                  (LocalVariables|SetTemp%20Card (Utilities|Array|Get(acopy) (Variables|Default|GetCurrent%20Hand) _index_4))
                  (Utilities|Array|SetArrayElem (Variables|Default|GetCurrent%20Hand) _index_4 (Utilities|Array|Get(acopy) (Variables|Default|GetCurrent%20Hand) (+ _index_4 1)))
                  (Utilities|Array|SetArrayElem (Variables|Default|GetCurrent%20Hand) (+ _index_4 1) (LocalVariables|GetTemp%20Card))))))
          (if (not (LocalVariables|GetSwapped))
            (goto _label_2 Break)))
        (:Completed
          (return))))
    (:NewEnumerator5
      ;[0 0 0] Randomises the current hand
      (Utilities|Array|Shuffle (Variables|Default|GetCurrent%20Hand))
      (return))))

(fn UpdateVisibleHand
  (params (Hand%20Spline :type Spline%20Component%20Object%20Reference) (Player? :type Boolean) (Player%20Camera :type Camera%20Component%20Object%20Reference))
  (bind _current_hand (Variables|Default|GetCurrent%20Hand))
  (Utilities|IsValid Hand%20Spline
    (:Is%20Valid
      (for (_array_element _array_index) _current_hand
        (if Player?
          (Default|MoveCardSmoothly _array_element (Spline|GetLocationatDistanceAlongSpline Hand%20Spline (* (/ (Spline|GetSplineLength Hand%20Spline) (- (Utilities|Array|Length _current_hand) 1)) _array_index) "World") (Transformation|GetWorldRotation Player%20Camera) 0.25 Player%20Camera Player%20Camera)
          (else
            (bind _returnvalue (Actor|GetActorOfClass "/Game/Player/BP_Player.BP_Player_C"))
            (Default|MoveCardSmoothly _array_element (Spline|GetLocationatDistanceAlongSpline Hand%20Spline (* (/ (Spline|GetSplineLength Hand%20Spline) (- (Utilities|Array|Length _current_hand) 1)) _array_index) "World") (Math|Rotator|SelectRotator "90.000000,0.000000,0.000000" (Math|Rotator|FindLookatRotation (Transformation|GetSocketLocation (Actor|GetComponentbyClass (Components|GetOwner) "/Script/Engine.SkeletalMeshComponent") "head") (Spline|GetLocationatDistanceAlongSpline Hand%20Spline (* (/ (Spline|GetSplineLength Hand%20Spline) (- (Utilities|Array|Length _current_hand) 1)) _array_index) "World")) (Variables|/Game/Player/BP_Player.BP_Player_C|GetZoom_In_Active _returnvalue)) 0.25 0 (Actor|GetComponentbyClass (Components|GetOwner) "/Script/Engine.CapsuleComponent")))))
      (Utilities|Time|SetTimerbyFunctionName 0 "Hover First Card" 0.25))
    (:Is%20Not%20Valid
      (Development|PrintString "HAND SPLINE NOT VALID FOR VISIBLE HAND"))))

(fn CanSelectCard
  (params (Card%20to%20Check :type BP%20Card%20Object%20Reference))
  (bind _selected_cards (Variables|Default|GetSelected%20Cards))
  ;[0 0 0] Consolidated functionality for checking if able to select a card
  (bind _returnvalue (Actor|GetActorOfClass "/Game/Main_Game_Managers/Auction/BP_Auction_Game_Manager.BP_Auction_Game_Manager_C"))
  (bind _asgm_bar (Utilities|Casting|CastToGM_Bar (Game|GetGameMode)))
  (if (Utilities|Array|ContainsItem _selected_cards Card%20to%20Check)
    (return false)
    (elif (> (Utilities|Array|Length _selected_cards) (Utilities|Select :Index (Variables|/Game/Modes_Instances/Modes/GM_Bar.GM_Bar_C|GetCurrent%20Playing%20Game _asgm_bar) :NewEnumerator0 3 :NewEnumerator1 (Math|Integer|SelectInt 1 (Math|Integer|SelectInt -1 0 (.ReturnValue (Utilities|Map|Find (Variables|/Game/Main_Game_Managers/Auction/BP_Auction_Game_Manager.BP_Auction_Game_Manager_C|GetPlayer%20w/%20War%20->%20Round _returnvalue) (Components|GetOwner)))) (.ReturnValue (Utilities|Map|Find (Variables|/Game/Main_Game_Managers/Auction/BP_Auction_Game_Manager.BP_Auction_Game_Manager_C|GetPlayer%20w/%20Conquest%20->%20Round _returnvalue) (Components|GetOwner)))) :NewEnumerator2 0 :NewEnumerator3 0 :NewEnumerator4 0 :NewEnumerator5 0))
      (return false)
      (else
        (return true)))))

(fn HoverFirstCard
  (Variables|Default|GetHovered%20Card
    (:then)
    (:else
      (if (not (Utilities|DoesObjectImplementInterface (Components|GetOwner) "/Game/NPCs/BPI_NPC_Opponent.BPI_NPC_Opponent_C"))
        (Hovering|HoverCheck (Utilities|Array|Get(acopy) (Variables|Default|GetCurrent%20Hand)))))))