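; Reusable dart projectile for the darts mini-game that is activated and deactivated rather than spawned or destroyed by its own logic.
; Activation places it at the throw position, aims it at the preferred end position, and launches it at the projectile movement's max speed.
; While active, a hit attaches it to the struck actor's root, keeping world transform.
; Deactivation detaches the mesh, moves the actor to world origin, disables collision and hides it.
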(event OnComponentHit(Dart_Sm)
  (params (HitComponent :type Primitive%20Component%20Object%20Reference) (OtherActor :type Actor%20Object%20Reference) (OtherComp :type Primitive%20Component%20Object%20Reference) (NormalImpulse :type Vector :default "0, 0, 0") (Hit :type Hit%20Result%20Structure%20%28by%20ref%29))
  (Development|PrintString (Utilities|GetDisplayName OtherActor))
  (if (Variables|Default|GetActive)
    (Transformation|AttachComponentToComponent (Variables|/Script/Engine.Actor|GetRootComponent OtherActor) "None" "KeepWorld" "KeepWorld" "KeepWorld" true)))

(event Custom|Deactivate%20Dart
  (Transformation|DetachFromComponent (Variables|Default|GetDart_Sm) "KeepWorld" "KeepWorld" "KeepWorld" true)
  (Variables|Default|SetActive false)
  (Development|PrintString "DEACTIVATED DART")
  (Transformation|SetActorLocation "0, 0, 0" false false)
  (Collision|SetActorEnableCollision false)
  (Rendering|SetActorHiddenInGame true))

(event Custom|Activate%20Dart
  (params (Throw%20Position :type Vector) (Preferred%20End%20Position :type Vector))
  (Transformation|SetActorLocationAndRotation Throw%20Position (Math|Rotator|FindLookatRotation Throw%20Position Preferred%20End%20Position))
  (Variables|Default|SetActive true)
  (Variables|/Script/Engine.MovementComponent|SetVelocity (Variables|Default|GetProjectileMovement) (* (Math|Vector|GetForwardVector (Transformation|GetActorRotation)) (Variables|/Script/Engine.ProjectileMovementComponent|GetMaxSpeed (Variables|Default|GetProjectileMovement))))
  (Components|Movement|SetUpdatedComponent (Variables|Default|GetProjectileMovement) (Variables|Default|GetDart_Sm))
  (Collision|SetActorEnableCollision true)
  (Rendering|SetActorHiddenInGame false))

(fn ConstructionScript)