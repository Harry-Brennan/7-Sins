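; Trigger actor for an outside loop that sends an overlapping actor to a loop end position behind a screen fade.
; On LoopCollision overlap it fades the camera to black, waits a configurable delay, then fades back in after relocating.
; The relocation copies LoopEndPosition's rotation to the player controller and moves the overlapping actor to its location.
; The overlap has no actor filter, while fade and rotation always target the player.
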(event OnComponentBeginOverlap(LoopCollision)
  (params (OverlappedComponent :type Primitive%20Component%20Object%20Reference) (OtherActor :type Actor%20Object%20Reference) (OtherComp :type Primitive%20Component%20Object%20Reference) (OtherBodyIndex :type Integer) (bFromSweep :type Boolean) (SweepResult :type Hit%20Result%20Structure%20%28by%20ref%29))
  (bind _loop_end_position (Variables|Default|GetLoop%20End%20Position))
  (bind _returnvalue (Transformation|GetActorTransform _loop_end_position))
  (bind (_location _rotation) (Math|Transform|BreakTransform _returnvalue))
  ;[0 0 0] Fade to black
  (CameraFades|StartCameraFade :self (Game|GetPlayerCameraManager 0) :ToAlpha 1.0 :Duration (Variables|Default|GetFade%20Time) :bHoldWhenFinished true)
  ;[0 0 0] Wait
  (Utilities|FlowControl|Delay (Variables|Default|GetTime%20before%20moving%20and%20fading%20in))
  ;[0 0 0] Set player position and location and then fade to alpha 0
  (Pawn|SetControlRotation (Game|GetPlayerController 0) _rotation)
  (Transformation|SetActorLocation OtherActor _location false false)
  (CameraFades|StartCameraFade :self (Game|GetPlayerCameraManager 0) :FromAlpha 1.0 :Duration (Variables|Default|GetFade%20Time)))

(fn ConstructionScript)