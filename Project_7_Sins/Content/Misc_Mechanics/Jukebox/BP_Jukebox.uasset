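; BP_Jukebox is an interactable world jukebox that plays a song list, with next, previous and fade-based pause and resume.
; Playback-percent updates track the resume time and advance to the next song when one ends.
; Overlapping the interaction radius enables the player's widget interaction and starts a looping timer that box-traces from the player's view.
; DoOnce gates use that trace to show or hide the WBP_Jukebox widget's buttons.
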(event OnComponentBeginOverlap(InteractCollisionRadius)
  (params (OverlappedComponent :type Primitive%20Component%20Object%20Reference) (OtherActor :type Actor%20Object%20Reference) (OtherComp :type Primitive%20Component%20Object%20Reference) (OtherBodyIndex :type Integer) (bFromSweep :type Boolean) (SweepResult :type Hit%20Result%20Structure%20%28by%20ref%29))
  (bind _player_ref (Variables|References|GetPlayer%20Ref))
  (bind _player_ref_2 (Variables|References|GetPlayer%20Ref))
  (bind _player_ref_3 (Variables|References|GetPlayer%20Ref))
  ;[0 0 0] Player interaction
  (Utilities|FlowControl|DoOnce false
    (:Completed
      (Utilities|FlowControl|Sequence
        (:then_0
          (Utilities|FlowControl|DoOnce false) ; enters at Reset
        )
        (:then_1
          (CallFunction|StartLineOfSight)
          (Variables|PlayerInteraction|SetPlayer%20In%20Range true)
          (Variables|/Game/Player/BP_Player.BP_Player_C|SetCan%20Interact%20With%20Jukebox _player_ref_2 true)
          (Components|Activation|Activate (Variables|/Game/Player/BP_Player.BP_Player_C|GetWidget%20Interaction _player_ref_2) false))))))

(event OnComponentEndOverlap(InteractCollisionRadius)
  (params (OverlappedComponent :type Primitive%20Component%20Object%20Reference) (OtherActor :type Actor%20Object%20Reference) (OtherComp :type Primitive%20Component%20Object%20Reference) (OtherBodyIndex :type Integer))
  (bind _player_ref (Variables|References|GetPlayer%20Ref))
  (bind _player_ref_2 (Variables|References|GetPlayer%20Ref))
  (bind _player_ref_3 (Variables|References|GetPlayer%20Ref))
  ;[0 0 0] Player interaction
  (Utilities|FlowControl|DoOnce false
    (:Completed
      (Utilities|FlowControl|Sequence
        (:then_0
          (Utilities|FlowControl|DoOnce false) ; enters at Reset
        )
        (:then_1
          (CallFunction|StopLineOfSight)
          (Variables|PlayerInteraction|SetPlayer%20In%20Range false)
          (Variables|/Game/Player/BP_Player.BP_Player_C|SetCan%20Interact%20With%20Jukebox _player_ref false)
          (if (and (Utilities|Array|IsEmpty (Collision|GetOverlappingActors _player_ref_3 "/Game/NPCs/BP_NPC.BP_NPC_C" :!class /Script/Engine.Actor)) (Utilities|Array|IsEmpty (Collision|GetOverlappingActors _player_ref_3 "/Game/Mini_Games/Darts/Dart_Board/BP_Dart_Board.BP_Dart_Board_C" :!class /Script/Engine.Actor)))
            (Components|Activation|Deactivate (Variables|/Game/Player/BP_Player.BP_Player_C|GetWidget%20Interaction _player_ref)))
          (CallFunction|HideUI))))))

(event Custom|Check%20Line%20of%20Sight
  (bind _player_ref (Variables|References|GetPlayer%20Ref))
  (bind _returnvalue (Pawn|GetControlRotation _player_ref :!class /Script/Engine.Pawn))
  (bind _outlocation (Actor|GetActorEyesViewPoint _player_ref))
  ;[0 0 0] Line of sight for player interaction and toggling the UI visibility
  (bind _returnvalue_2 (Class|KismetSystemLibrary|BoxTraceSingleforObjects _outlocation (+ (* (Math|Vector|GetForwardVector _returnvalue) 5e+02) _outlocation) "64.000000,64.000000,64.000000" _returnvalue (Utilities|Array|MakeArray "ObjectTypeQuery10") false 0 "None" false))
  (if _returnvalue_2
    (if (Variables|PlayerInteraction|GetPlayer%20In%20Range)
      (Utilities|FlowControl|DoOnce false :!label _label
        (:Completed
          (Utilities|FlowControl|Sequence
            (:then_0
              (CallFunction|ShowUI))
            (:then_1
              (goto _label_3 Reset)))))
      (else
        (Utilities|FlowControl|Sequence :!label _label_2
          (:then_0
            (goto _label Reset))
          (:then_1
            (Utilities|FlowControl|DoOnce false :!label _label_3
              (:Completed
                (CallFunction|HideUI)))))))
    (else
      (goto _label_2))))

(event Custom|Start%20Line%20Of%20Sight
  ;[0 0 0] Line of sight for player interaction and toggling the UI visibility
  (bind _returnvalue (Utilities|Time|SetTimerbyEvent (delegate Custom|Check%20Line%20of%20Sight) 0.05 true)))

(event Custom|Stop%20Line%20Of%20Sight
  ;[0 0 0] Line of sight for player interaction and toggling the UI visibility
  (Utilities|Time|ClearandInvalidateTimerbyHandle (stale Custom|Start%20Line%20Of%20Sight _returnvalue))
  (Utilities|FlowControl|DoOnce false) ; enters at Reset
)

(event Custom|Show%20UI
  ;[0 0 0] Toggle hide and show UI visibiltiy
  (Rendering|SetVisibility (Variables|Default|GetJukebox%20UI) true false)
  (Default|ShowButtons (Variables|References|GetJukebox%20Widget%20Ref)))

(event Custom|Hide%20UI
  ;[0 0 0] Toggle hide and show UI visibiltiy
  (Default|HideButtons (Variables|References|GetJukebox%20Widget%20Ref))
  (Utilities|FlowControl|Delay 0.25)
  (if (not (Variables|PlayerInteraction|GetPlayer%20In%20Range))
    (Rendering|SetVisibility (Variables|Default|GetJukebox%20UI) false false)))

(event Custom|Playback%20Update
  (params (PlayingSoundWave :type Sound%20Wave%20Object%20Reference) (PlaybackPercent :type Float%20%28single-precision%29))
  ;[0 0 0] Setup player ref and set off the tick for event for getting the playback percent of the audio and checking if it is greater than 1 meaning the audio has reached its end then we call next song this is also where we set the audio time which is used when resuming a song
  (if (>= PlaybackPercent 1.0)
    (CallFunction|NextSong)
    (else
      (Variables|Songs|SetAudio%20Time (* PlaybackPercent (Variables|/Script/Engine.SoundBase|GetDuration PlayingSoundWave))))))

(event Custom|Pause%20/%20Unpause%20Song
  ;[0 0 0] Gate for pausing and unpausing the audio - will probably change this to some fade out and fade in as well
  (if (Variables|Songs|GetPaused)
    (Audio|Components|Audio|FadeIn (Variables|Default|GetAudio) (Variables|FadeTimes|GetFade%20In%20Time) 1.0 (Variables|Songs|GetAudio%20Time) "Linear" :!class /Script/Engine.AudioComponent)
    (else
      (Audio|Components|Audio|FadeOut (Variables|Default|GetAudio) (Variables|FadeTimes|GetFade%20Out%20Time) 0.0 "Linear" :!class /Script/Engine.AudioComponent))))

(event Custom|Next%20Song
  (bind _songs (Variables|Songs|GetSongs))
  (bind _returnvalue (Utilities|Array|LastIndex _songs))
  ;[0 0 0] Next and previous song functions
  (Development|PrintString "NEXT SONG")
  (bind _output_get (Variables|Songs|SetCurrent%20Song%20Index (Math|Integer|SelectInt _returnvalue (+ (Variables|Songs|GetCurrent%20Song%20Index) 1) (> (+ (Variables|Songs|GetCurrent%20Song%20Index) 1) _returnvalue))))
  (Audio|Components|Audio|SetSound (Variables|Default|GetAudio) (Utilities|Array|Get(acopy) (Variables|Songs|GetSongs) _output_get))
  (Audio|Components|Audio|FadeIn (Variables|Default|GetAudio) (Variables|FadeTimes|GetFade%20In%20Time) 1.0 0.0 "Linear" :!class /Script/Engine.AudioComponent)
  (Variables|Songs|SetPaused false))

(event Custom|Previous%20Song
  ;[0 0 0] Next and previous song functions
  (Development|PrintString "PREVIOUS SONG")
  (bind _output_get (Variables|Songs|SetCurrent%20Song%20Index (Math|Integer|SelectInt (Utilities|Array|LastIndex (Variables|Songs|GetSongs)) (- (Variables|Songs|GetCurrent%20Song%20Index) 1) (< (- (Variables|Songs|GetCurrent%20Song%20Index) 1) 0))))
  (Audio|Components|Audio|SetSound (Variables|Default|GetAudio) (Utilities|Array|Get(acopy) (Variables|Songs|GetSongs) _output_get))
  (Audio|Components|Audio|FadeIn (Variables|Default|GetAudio) (Variables|FadeTimes|GetFade%20In%20Time) 1.0 0.0 "Linear" :!class /Script/Engine.AudioComponent)
  (Variables|Songs|SetPaused false))

(event EventBeginPlay
  ;[0 0 0] Setup player ref and set off the tick for event for getting the playback percent of the audio and checking if it is greater than 1 meaning the audio has reached its end then we call next song this is also where we set the audio time which is used when resuming a song
  (bind _returnvalue (Actor|GetActorOfClass "/Game/Player/BP_Player.BP_Player_C"))
  (Variables|References|SetPlayer%20Ref _returnvalue)
  (EventDispatchers|BindEventtoOnAudioPlaybackPercent (Variables|Default|GetAudio) (delegate Custom|Playback%20Update))
  (Audio|Components|Audio|FadeIn (Variables|Default|GetAudio) (Variables|FadeTimes|GetFade%20In%20Time) 1.0 0.0 "Linear" :!class /Script/Engine.AudioComponent)
  (bind _aswbp_jukebox (Utilities|Casting|CastToWBP_Jukebox (UserInterface|GetWidget (Variables|Default|GetJukebox%20UI))))
  (Variables|References|SetJukebox%20Widget%20Ref _aswbp_jukebox))

(fn ConstructionScript)