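; Card pile actor that holds an ordered array of cards and displays them as a visible stack in a card game.
; AddCard offsets each card along the StackDirection arrow's forward vector, while removal hides the card at world origin and restacks those above it.
; ClearCardPile hides and empties the pile, and OutSlapInfo exposes the last three cards and the first for slap checks.
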(fn ConstructionScript)

(fn AddCard
  (params (Card :type BP%20Card%20Object%20Reference) (Debug :type Boolean))
  ;[1 1 1] Add the passed card to the cardsinile array
  (bind _returnvalue (Utilities|Array|Add (Variables|Default|GetCardsInPile) Card))
  ;[1 1 1] Debug message for what card is being added to what pile
  (Development|PrintString (Utilities|String|Append (Utilities|GetDisplayName Card) " IS BEING ADDED TO THE " (Utilities|GetDisplayName self)) Debug Debug "(R=0.023588,G=0.000000,B=1.000000,A=1.000000)" 1e+02)
  ;[1 1 1] Set the card location to be the above the previous card's location by a set amount using forward vector of the stacking direction arrow and also set the rotation to be the rotation of the pile and set this card visible as well
  ;;[1 1 1] If it is the first card to be added
  (if (== _returnvalue 0)
    ;[1 1 1] Set card location to be the location of the pile and the rotation of the pile and set it visible
    (Transformation|SetActorLocationAndRotation Card (Transformation|GetActorLocation) (Utilities|CardRotation))
    (Rendering|SetActorHiddenInGame Card false)
    (else
      (Transformation|SetActorLocationAndRotation Card (+ (Transformation|GetActorLocation) (* (Math|Vector|GetForwardVector (Variables|Default|GetStack%20Direction)) (* (- (Utilities|Array|Length (Variables|Default|GetCardsInPile)) 1) (Variables|Default|GetCard%20Stack%20Amount)))) (Utilities|CardRotation))
      (Rendering|SetActorHiddenInGame Card false)))
  ;[1 1 1] Debug printing what card is being added to the pile
  (bind _card_info (Default|GetCardInfo Card))
  (Development|PrintString (Utilities|String|Append (Utilities|String|EnumtoString (.CardName (Utilities|Struct|BreakStruct_Card _card_info))) " of " (Utilities|String|EnumtoString (.Suit (Utilities|Struct|BreakStruct_Card _card_info))) " added to:" (Utilities|GetDisplayName self) " which is card: " (Utilities|GetDisplayName Card)) Debug Debug))

(fn ClearCardPile
  ;[1 1 1] Clears all the cards in the pile setting them hidden as well
  (for _array_element (Variables|Default|GetCardsInPile)
    (Rendering|SetActorHiddenInGame _array_element true))
  (Utilities|Array|Clear (Variables|Default|GetCardsInPile)))

(fn RemoveCardfromVisualPile
  (params (Card :type BP%20Card%20Object%20Reference))
  ;[1 1 1] Removes card from the pile array - other functions move the card around so use those after this
  (LocalVariables|SetCard%20To%20Remove%20Index (Utilities|Array|FindItem (Variables|Default|GetCardsInPile) Card))
  ;[1 1 1] Debug message
  (Utilities|Array|RemoveItem (Variables|Default|GetCardsInPile) Card)
  (Development|PrintString (Utilities|String|Append (Utilities|GetDisplayName Card) " being removed from the pile in the " (Utilities|GetDisplayName self)) true true "(R=0.000000,G=1.000000,B=0.027025,A=1.000000)" 1e+02)
  ;[1 1 1] Set to 0,0,0 and set hidden
  (Transformation|SetActorLocation Card "0, 0, 0" false false)
  (Rendering|SetActorHiddenInGame Card true)
  ;[1 1 1] Only loop through the cards to adjust positions and rotations if the card that was removed wasn't the top card
  (if (not (== (LocalVariables|GetCard%20To%20Remove%20Index) (Utilities|Array|Length (Variables|Default|GetCardsInPile))))
    (for (_array_element _array_index) (Variables|Default|GetCardsInPile)
      ;[1 1 1] Set to current card in loop
      (LocalVariables|SetCurrent%20Looping%20Card _array_element)
      ;[1 1 1] Set the card location to be the above the previous card's location by a set amount using forward vector of the stacking direction arrow and also set the rotation to be the rotation of the pile and set this card visible as well
      ;;[1 1 1] Only changing position if the card is above the card that was removed in order
      (if (>= _array_index (LocalVariables|GetCard%20To%20Remove%20Index))
        ;;[1 1 1] if it is the first card in the pile
        (if (== _array_index 0)
          ;[1 1 1] Set card location to be the location of the pile and the rotation of the pile and set it visible
          (Transformation|SetActorLocationAndRotation (LocalVariables|GetCurrent%20Looping%20Card) (Transformation|GetActorLocation) (Utilities|CardRotation))
          (Rendering|SetActorHiddenInGame (LocalVariables|GetCurrent%20Looping%20Card) false)
          (else
            (Transformation|SetActorLocationAndRotation (LocalVariables|GetCurrent%20Looping%20Card) (+ (Transformation|GetActorLocation) (* (Math|Vector|GetForwardVector (Variables|Default|GetStack%20Direction)) (* _array_index (Variables|Default|GetCard%20Stack%20Amount)))) (Utilities|CardRotation))
            (Rendering|SetActorHiddenInGame (LocalVariables|GetCurrent%20Looping%20Card) false)))))))

(fn OutSlapInfo
  (bind _cardsinpile (Variables|Default|GetCardsInPile))
  (return (Utilities|Array|Get(acopy) _cardsinpile (Utilities|Array|LastIndex _cardsinpile)) (Utilities|Array|Get(acopy) _cardsinpile (- (Utilities|Array|LastIndex _cardsinpile) 1)) (Utilities|Array|Get(acopy) _cardsinpile (- (Utilities|Array|LastIndex _cardsinpile) 2)) (Utilities|Array|Get(acopy) _cardsinpile)))