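; BP_Card_Dealer builds, shuffles and deals the deck for three card games: I Doubt It, Auction and Rat Screw.
; BeginPlay spawns a hidden BP_Card per DT_Cards row and caches the game managers.
; SetupCards splits cards into player and pile arrays by game; DealCards deals round-robin for I Doubt It or into two piles for Rat Screw, with no Auction case.
; Helpers update these arrays alongside hands and pile actors.
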(event EventBeginPlay
  ;[1 1 1] Get all card names
  (Utilities|FlowControl|Sequence
    (:then_0
      (bind _outrownames (DataTable|GetDataTableRowNames "/Game/Shared_Game_Mechanics/Cards/DT_Cards.DT_Cards"))
      ;[1 1 1] Loop through all cards
      (for _array_element _outrownames
        ;[1 1 1] Get info of current card name
        (bind _returnvalue (Utilities|GetDataTableRow "/Game/Shared_Game_Mechanics/Cards/DT_Cards.DT_Cards" _array_element)
          (:then
            ;[1 1 1] Spawn card passing out row as card info
            (bind _returnvalue_2 (Game|SpawnActorfromClass "/Game/Shared_Game_Mechanics/Cards/BP_Card.BP_Card_C" (Math|Transform|MakeTransform "0, 0, 0" "0, 0, 0" "1.000000,1.000000,1.000000") "Undefined" "MultiplyWithRoot" 0 _returnvalue 0))
            ;[1 1 1] Set card hidden and collision disabled
            (Rendering|SetActorHiddenInGame _returnvalue_2 true)
            (Collision|SetActorEnableCollision _returnvalue_2 false)
            ;[1 1 1] Add spawned card to all cards array
            (Utilities|Array|Add (Variables|Default|GetAll%20Cards) _returnvalue_2)))))
    (:then_1
      ;[1 1 1] Get references to all game managers
      (bind _returnvalue_3 (Actor|GetActorOfClass "/Game/Main_Game_Managers/Auction/BP_Auction_Game_Manager.BP_Auction_Game_Manager_C"))
      (Variables|Default|SetAuctionManager _returnvalue_3)
      (bind _returnvalue_4 (Actor|GetActorOfClass "/Game/Main_Game_Managers/Rat_Screw/BP_Rat_Screw_Game_Manager.BP_Rat_Screw_Game_Manager_C"))
      (Variables|Default|SetRatScrewManager _returnvalue_4)
      (bind _returnvalue_5 (Actor|GetActorOfClass "/Game/Main_Game_Managers/I_Doubt_It/BP_I_Doubt_It_Game_Manager.BP_I_Doubt_It_Game_Manager_C"))
      (Variables|Default|SetIDoubtItManager _returnvalue_5))))

(fn ConstructionScript)

(fn SetupCards
  (params (Game%20Name :type Enum_Main_Game_Names%20Enum :default "NewEnumerator0"))
  ;[1 1 1] Pass the main game name to this function
  (switch Utilities|FlowControl|Switch|SwitchonEnum_Main_Game_Names Game%20Name
    (:NewEnumerator0
      ;[1 1 1] Set the player cards to be all the cards spawned and clear the pile cards since I doubt it doesn't have any pile cards at the start of the game
      (Variables|Default|SetPlayer%20Cards (Variables|Default|GetAll%20Cards))
      (Utilities|Array|Clear (Variables|Default|GetPile%20Cards)))
    (:NewEnumerator1
      ;[1 1 1] Loop through all the cards
      (for _array_element (Variables|Default|GetAll%20Cards)
        ;[1 1 1] Get the card's info and then get the card's numerical value
        (bind _card_info (Class|BPICard|GetCardInfo(Message) _array_element))
        ;[1 1 1] If it is between these values then add to the player cards
        (if (and (> (.NumericalValue (Utilities|Struct|BreakStruct_Card _card_info)) 1) (< (.NumericalValue (Utilities|Struct|BreakStruct_Card _card_info)) 11))
          (Utilities|Array|Add (Variables|Default|GetPlayer%20Cards) _array_element)
          (else
            ;[1 1 1] If it is a different card add it to the pile cards array
            (Utilities|Array|Add (Variables|Default|GetPile%20Cards) _array_element)))))
    (:NewEnumerator2
      ;[1 1 1] Set the player cards to be all the cards spawned and clear the pile cards since Rat Screw doesn't have any pile cards at the start of the game
      (Variables|Default|SetPlayer%20Cards (Variables|Default|GetAll%20Cards))
      (Utilities|Array|Clear (Variables|Default|GetPile%20Cards)))))

(fn ShuffleCards
  ;[1 1 1] If the pile cards array is not empty then shuffle it
  (if (Utilities|Array|IsEmpty (Variables|Default|GetPile%20Cards))
    _
    (else
      (Utilities|Array|Shuffle (Variables|Default|GetPile%20Cards))))
  ;[1 1 1] Shuffle the cards that players will have
  (Utilities|Array|Shuffle (Variables|Default|GetPlayer%20Cards)))

(fn DealCards
  (params (Game%20Name :type Enum_Main_Game_Names%20Enum :default "NewEnumerator0") (Players :type Array%20of%20Actor%20Object%20References))
  ;[1 1 1] Pass the main game name and the players in the game
  ;[1 1 1] Switch based on the game name
  (switch Utilities|FlowControl|Switch|SwitchonEnum_Main_Game_Names Game%20Name
    (:NewEnumerator0
      ;[1 1 1] Reset current card deal index eventhough its a local variable
      (LocalVariables|SetCurrent%20Card%20Deal%20Index 0)
      (for _index (range 1 (/ (Utilities|Array|Length (Variables|Default|GetPlayer%20Cards)) (Utilities|Array|Length Players)))
        ;[1 1 1] loop players
        (for _array_element Players
          ;[1 1 1] Add card to each player one after another as if a real card dealer dealing to each player one after another with one card at a time
          (CallFunction|AddCardtoPlayerHand _array_element (Utilities|Array|Get(acopy) (Variables|Default|GetPlayer%20Cards) (LocalVariables|GetCurrent%20Card%20Deal%20Index)))
          (Math|Integer|IncrementInt (LocalVariables|GetCurrent%20Card%20Deal%20Index)))))
    (:NewEnumerator2
      ;[1 1 1] Loop through the first 30 cards of the deck and add them to the player's pile.
      (LocalVariables|SetCurrent%20Card%20Deal%20Index 0)
      (for _index_2 (range 1 30)
        (CallFunction|AddCardtoPile (Utilities|Array|Get(acopy) (Variables|Default|GetPlayer%20Cards) (LocalVariables|GetCurrent%20Card%20Deal%20Index)) (Variables|/Game/Main_Game_Managers/Rat_Screw/BP_Rat_Screw_Game_Manager.BP_Rat_Screw_Game_Manager_C|GetPlayerCardPIle (Variables|Default|GetRatScrewManager)) true)
        (Math|Integer|IncrementInt (LocalVariables|GetCurrent%20Card%20Deal%20Index)))
      ;[1 1 1] Deal the remaining cards to the opponent
      (for _index_3 (range 31 60)
        (CallFunction|AddCardtoPile (Utilities|Array|Get(acopy) (Variables|Default|GetPlayer%20Cards) (LocalVariables|GetCurrent%20Card%20Deal%20Index)) (Variables|/Game/Main_Game_Managers/Rat_Screw/BP_Rat_Screw_Game_Manager.BP_Rat_Screw_Game_Manager_C|GetOpponentCardPile (Variables|Default|GetRatScrewManager)) true)
        (Math|Integer|IncrementInt (LocalVariables|GetCurrent%20Card%20Deal%20Index)))
      (Development|PrintString (Utilities|String|ToString(Integer) (Utilities|Array|Length (Variables|/Game/Shared_Game_Mechanics/Cards/BP_CardPile.BP_CardPile_C|GetCardsInPile (Variables|/Game/Main_Game_Managers/Rat_Screw/BP_Rat_Screw_Game_Manager.BP_Rat_Screw_Game_Manager_C|GetOpponentCardPile (Variables|Default|GetRatScrewManager))))))
      (Development|PrintString (Utilities|String|ToString(Integer) (Utilities|Array|Length (Variables|/Game/Shared_Game_Mechanics/Cards/BP_CardPile.BP_CardPile_C|GetCardsInPile (Variables|/Game/Main_Game_Managers/Rat_Screw/BP_Rat_Screw_Game_Manager.BP_Rat_Screw_Game_Manager_C|GetPlayerCardPIle (Variables|Default|GetRatScrewManager)))))))))

(fn AddCardtoPile
  (params (Card :type BP%20Card%20Object%20Reference) (Which%20Pile :type BP%20Card%20Pile%20Object%20Reference) (Debug :type Boolean))
  ;[1 1 1] Adding a card to the pile array
  (Utilities|Array|Add (Variables|Default|GetPile%20Cards) Card)
  ;[1 1 1] Add card to the passed pile actor
  (Default|AddCard Which%20Pile Card Debug))

(fn RemoveCardfromPile
  (params (Card%20to%20Remove%20From%20Pile :type BP%20Card%20Object%20Reference) (Pile%20To%20Remove%20From :type BP%20Card%20Pile%20Object%20Reference))
  ;[1 1 1] Remove a card from the pile array
  (Utilities|Array|RemoveItem (Variables|Default|GetPile%20Cards) Card%20to%20Remove%20From%20Pile)
  ;[1 1 1] Remove card from the pile array in the specific pile
  (Default|RemoveCardfromVisualPile Pile%20To%20Remove%20From Card%20to%20Remove%20From%20Pile))

(fn AddCardtoPlayerHand
  (params (Character :type Actor%20Object%20Reference) (Card :type BP%20Card%20Object%20Reference))
  (bind _player_cards (Variables|Default|GetPlayer%20Cards))
  ;[1 1 1] Add the passed card to the passed character's hand
  (Class|BPIPlayingCharacter|AddCardtoHand(Message) Character Card)
  (if (not (Utilities|Array|ContainsItem _player_cards Card))
    ;[1 1 1] Add passed to player cards array
    (Utilities|Array|Add _player_cards Card)))

(fn RemoveCardfromPlayerHand
  (params (Character :type Actor%20Object%20Reference) (Card :type BP%20Card%20Object%20Reference))
  ;[1 1 1] Remove the passed card from the passed character's hand
  (Class|BPIPlayingCharacter|RemoveCardfromHand(Message) Character Card)
  ;[1 1 1] Remove passed card from player cards array
  (Utilities|Array|RemoveItem (Variables|Default|GetPlayer%20Cards) Card))

(fn ClearCardPile
  (params (Card%20Pile :type BP%20Card%20Pile%20Object%20Reference))
  (Utilities|Array|Clear (Variables|Default|GetPile%20Cards))
  (Default|ClearCardPile Card%20Pile))