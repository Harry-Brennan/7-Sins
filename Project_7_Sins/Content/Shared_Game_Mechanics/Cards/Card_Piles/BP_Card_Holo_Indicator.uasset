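; BP_Card_Holo_Indicator is a semi-transparent "holo" card that displays the mesh and identity held in its CardInfo struct.
; The construction script and UpdateInfo repeat the same setup: set the mesh, apply a test material, and write name and suit to a text render for debugging.
; Each run creates a dynamic material instance with a random colour, with UpdateInfo using a lower alpha than construction.
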(fn ConstructionScript
  (bind _card_info (Variables|Default|GetCard%20Info))
  (bind (_cardname _staticmesh _numericalvalue _suit) (Utilities|Struct|BreakStruct_Card _card_info))
  ;[0 0 0] Set card static mesh to be the static mesh from its info struct
  (Components|StaticMesh|SetStaticMesh (Variables|Default|GetHolo%20Card%20Mesh) (Utilities|Struct|BreakStruct_Card (Variables|Default|GetCard%20Info)))
  ;[0 0 0] Set material and debug text with the material as 0.25 alpha so slightly holo
  (bind _returnvalue (Rendering|Material|CreateDynamicMaterialInstance "/Game/Shared_Game_Mechanics/Cards/Materials/M_Card_Test.M_Card_Test" "None" "None" :!class /Script/Engine.KismetMaterialLibrary))
  (Rendering|Material|SetVectorParameterValue _returnvalue "Colour" (Utilities|Struct|MakeLinearColor (Math|Random|RandomFloat) (Math|Random|RandomFloat) (Math|Random|RandomFloat) 0.5) :!class /Script/Engine.MaterialInstanceDynamic)
  (Rendering|Material|SetMaterial (Variables|Default|GetHolo%20Card%20Mesh) 0 _returnvalue)
  (Rendering|Components|TextRender|SetText (Variables|Default|GetTextRender) (Utilities|Text|ToText(String) (Utilities|String|Append (Utilities|String|EnumtoString _cardname) " 
of 
" (Utilities|String|EnumtoString _suit)))))

(fn UpdateInfo
  (bind _card_info (Variables|Default|GetCard%20Info))
  (bind (_cardname _staticmesh _numericalvalue _suit) (Utilities|Struct|BreakStruct_Card _card_info))
  ;[0 0 0] Set card static mesh to be the static mesh from its info struct
  (Components|StaticMesh|SetStaticMesh (Variables|Default|GetHolo%20Card%20Mesh) (Utilities|Struct|BreakStruct_Card (Variables|Default|GetCard%20Info)))
  ;[0 0 0] Set material and debug text with the material as 0.25 alpha so slightly holo
  (bind _returnvalue (Rendering|Material|CreateDynamicMaterialInstance "/Game/Shared_Game_Mechanics/Cards/Materials/M_Card_Test.M_Card_Test" "None" "None" :!class /Script/Engine.KismetMaterialLibrary))
  (Rendering|Material|SetVectorParameterValue _returnvalue "Colour" (Utilities|Struct|MakeLinearColor (Math|Random|RandomFloat) (Math|Random|RandomFloat) (Math|Random|RandomFloat) 0.25) :!class /Script/Engine.MaterialInstanceDynamic)
  (Rendering|Material|SetMaterial (Variables|Default|GetHolo%20Card%20Mesh) 0 _returnvalue)
  (Rendering|Components|TextRender|SetText (Variables|Default|GetTextRender) (Utilities|Text|ToText(String) (Utilities|String|Append (Utilities|String|EnumtoString _cardname) " 
of 
" (Utilities|String|EnumtoString _suit)))))