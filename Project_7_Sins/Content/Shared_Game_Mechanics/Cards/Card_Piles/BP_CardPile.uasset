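; BP_CardPile is a card pile actor that holds an ordered array of cards and displays them as a physical stack.
; Adding or removing cards smoothly moves them to offsets along the StackDirection arrow, and clearing hides them all.
; AddCard can show a holographic child-actor indicator of the added card, which a looping timer keeps rotated toward the player.
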(fn ConstructionScript)

(fn AddCard
  (params (Card :type BP%20Card%20Object%20Reference) (Debug :type Boolean) (Show%20Holo? :type Boolean))
  ;[0 0 0] Add the passed card to the cardsinpile array
  (bind _returnvalue (Utilities|Array|Add (Variables|Default|GetCardsInPile) Card))
  ;[0 0 0] Card holo representation
  (if Show%20Holo?
    (CallFunction|ShowHoloCardRep (Variables|/Game/Shared_Game_Mechanics/Cards/BP_Card.BP_Card_C|GetCard%20Info Card))
    (else
      (CallFunction|HideHoloCardRep)))
  ;[0 0 0] Debug message for what card is being added to what pile
  (Development|PrintString (Utilities|String|Append (Utilities|GetDisplayName Card) " IS BEING ADDED TO THE " (Utilities|GetDisplayName self)) Debug Debug "(R=0.023588,G=0.000000,B=1.000000,A=1.000000)" 1e+02)
  ;[0 0 0] Set the card location to be the above the previous card's location by a set amount using forward vector of the stacking direction arrow and also set the rotation to be the rotation of the pile and set this card visible as well
  ;;[0 0 0] If it is the first card to be added
  (if (== _returnvalue 0)
    ;[0 0 0] Set card location to be the location of the pile and the rotation of the pile and set it visible
    (Class|BPICard|MoveCardSmoothly(Message) Card (Transformation|GetActorLocation) (Utilities|CardRotation) 0.5)
    (Rendering|SetActorHiddenInGame Card false)
    (else
      (Class|BPICard|MoveCardSmoothly(Message) Card (+ (Transformation|GetActorLocation) (* (Math|Vector|GetForwardVector (Variables|Default|GetStack%20Direction)) (* (- (Utilities|Array|Length (Variables|Default|GetCardsInPile)) 1) (Variables|Default|GetCard%20Stack%20Amount)))) (Utilities|CardRotation) 0.5)
      (Rendering|SetActorHiddenInGame Card false)))
  ;[0 0 0] Debug printing what card is being added to the pile
  (bind _card_info (Default|GetCardInfo Card))
  (Development|PrintString (Utilities|String|Append (Utilities|String|EnumtoString (.CardName (Utilities|Struct|BreakStruct_Card _card_info))) " of " (Utilities|String|EnumtoString (.Suit (Utilities|Struct|BreakStruct_Card _card_info))) " added to:" (Utilities|GetDisplayName self) " which is card: " (Utilities|GetDisplayName Card)) Debug Debug "(R=1.000000,G=0.000000,B=0.014380,A=1.000000)" 1e+02))

(fn ClearCardPile
  ;[0 0 0] Clears all the cards in the pile setting them hidden as well
  (for _array_element (Variables|Default|GetCardsInPile)
    (Rendering|SetActorHiddenInGame _array_element true))
  (Utilities|Array|Clear (Variables|Default|GetCardsInPile)))

(fn RemoveCardfromVisualPile
  (params (Card :type BP%20Card%20Object%20Reference))
  ;[0 0 0] Removes card from the pile array - other functions move the card around so use those after this
  (LocalVariables|SetCard%20To%20Remove%20Index (Utilities|Array|FindItem (Variables|Default|GetCardsInPile) Card))
  ;[0 0 0] Debug message
  (Utilities|Array|RemoveItem (Variables|Default|GetCardsInPile) Card)
  ;[0 0 0] Only loop through the cards to adjust positions and rotations if the card that was removed wasn't the top card
  (if (not (== (LocalVariables|GetCard%20To%20Remove%20Index) (Utilities|Array|Length (Variables|Default|GetCardsInPile))))
    (for (_array_element _array_index) (Variables|Default|GetCardsInPile)
      ;[0 0 0] Set to current card in loop
      (LocalVariables|SetCurrent%20Looping%20Card _array_element)
      ;[0 0 0] Set the card location to be the above the previous card's location by a set amount using forward vector of the stacking direction arrow and also set the rotation to be the rotation of the pile and set this card visible as well
      ;;[0 0 0] Only changing position if the card is above the card that was removed in order
      (if (>= _array_index (LocalVariables|GetCard%20To%20Remove%20Index))
        ;;[0 0 0] if it is the first card in the pile
        (if (== _array_index 0)
          ;[0 0 0] Set card location to be the location of the pile and the rotation of the pile and set it visible
          (Class|BPICard|MoveCardSmoothly(Message) (LocalVariables|GetCurrent%20Looping%20Card) (Transformation|GetActorLocation) (Utilities|CardRotation) 0.5)
          (else
            (Class|BPICard|MoveCardSmoothly(Message) (LocalVariables|GetCurrent%20Looping%20Card) (+ (Transformation|GetActorLocation) (* (Math|Vector|GetForwardVector (Variables|Default|GetStack%20Direction)) (* _array_index (Variables|Default|GetCard%20Stack%20Amount)))) (Utilities|CardRotation) 0.5)))))))

(fn AddCardtoBottom
  (params (Card :type BP%20Card%20Object%20Reference) (Debug :type Boolean))
  ;[0 0 0] Add the passed card to the cardsinile array
  (Utilities|Array|Insert (Variables|Default|GetCardsInPile) Card)
  ;[0 0 0] Debug message for what card is being added to what pile
  (Development|PrintString (Utilities|String|Append (Utilities|GetDisplayName Card) " IS BEING ADDED TO THE " (Utilities|GetDisplayName self)) Debug Debug "(R=0.023588,G=0.000000,B=1.000000,A=1.000000)" 1e+02)
  ;[0 0 0] Set the card location to be the above the previous card's location by a set amount using forward vector of the stacking direction arrow and also set the rotation to be the rotation of the pile and set this card visible as well
  (Class|BPICard|MoveCardSmoothly(Message) Card (+ (Transformation|GetActorLocation) (* (Math|Vector|GetForwardVector (Variables|Default|GetStack%20Direction)) (* (- (Utilities|Array|Length (Variables|Default|GetCardsInPile)) 1) (Variables|Default|GetCard%20Stack%20Amount)))) (Utilities|CardRotation) 0.5)
  (Rendering|SetActorHiddenInGame Card false)
  ;[0 0 0] Debug printing what card is being added to the pile
  (bind _card_info (Default|GetCardInfo Card))
  (Development|PrintString (Utilities|String|Append (Utilities|String|EnumtoString (.CardName (Utilities|Struct|BreakStruct_Card _card_info))) " of " (Utilities|String|EnumtoString (.Suit (Utilities|Struct|BreakStruct_Card _card_info))) " added to:" (Utilities|GetDisplayName self) " which is card: " (Utilities|GetDisplayName Card)) Debug Debug "(R=1.000000,G=0.000000,B=0.014380,A=1.000000)" 1e+02))

(fn ShowHoloCardRep
  (params (Card%20Info :type Struct%20Card%20Structure))
  (Development|SetHiddeninGame (Variables|Default|GetHolo%20Card) false false)
  (Utilities|IsValid (Variables|Default|GetPlayer%20Rep)
    (:Is%20Valid
      _)
    (:Is%20Not%20Valid
      (bind _returnvalue (Actor|GetActorOfClass "/Game/Player/BP_Player.BP_Player_C"))
      (Variables|Default|SetPlayer%20Rep _returnvalue)))
  (bind _asbp_card_holo_indicator (Utilities|Casting|CastToBP_Card_Holo_Indicator (Variables|/Script/Engine.ChildActorComponent|GetChildActor (Variables|Default|GetHolo%20Card))))
  (Variables|/Game/Shared_Game_Mechanics/Cards/Card_Piles/BP_Card_Holo_Indicator.BP_Card_Holo_Indicator_C|SetCard%20Info _asbp_card_holo_indicator Card%20Info)
  (Default|UpdateInfo _asbp_card_holo_indicator)
  (bind _returnvalue_2 (Utilities|Time|SetTimerbyFunctionName 0 "Rotate Holo To Player" 0.01 true))
  (Variables|Default|SetRotate%20Holo%20Card%20Timer _returnvalue_2))

(fn HideHoloCardRep
  (Development|SetHiddeninGame (Variables|Default|GetHolo%20Card) true false)
  (Utilities|Time|ClearandInvalidateTimerbyHandle (Variables|Default|GetRotate%20Holo%20Card%20Timer)))

(fn RotateHolotoPlayer
  (Transformation|SetWorldRotation (Variables|Default|GetHolo%20Card) (Math|Rotator|FindLookatRotation (Transformation|GetWorldLocation (Variables|Default|GetHolo%20Card)) (Transformation|GetActorLocation (Variables|Default|GetPlayer%20Rep))) false false))