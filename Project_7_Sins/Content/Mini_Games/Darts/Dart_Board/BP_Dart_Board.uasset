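; Dart board actor for the darts mini-game, hosting its world-space start, mode, difficulty, scoreboard, winner and aim-bar widgets.
; While the player is in range and no game is active, a looping timer box-traces from their view to toggle the start UI and widget interaction.
; Aiming runs horizontal then vertical sliders, storing both stopped values before telling BP_Dart_Game_Manager to play the dart.
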(event OnComponentBeginOverlap(InteractCollision)
  (params (OverlappedComponent :type Primitive%20Component%20Object%20Reference) (OtherActor :type Actor%20Object%20Reference) (OtherComp :type Primitive%20Component%20Object%20Reference) (OtherBodyIndex :type Integer) (bFromSweep :type Boolean) (SweepResult :type Hit%20Result%20Structure%20%28by%20ref%29))
  ;[0 0 0] Interaction collision for starting line of sight and also only doing starting line of sight if darts game is not already active
  (if (Variables|/Game/Mini_Games/Darts/BP_Dart_Game_Manager.BP_Dart_Game_Manager_C|GetDarts%20Game%20Active (Variables|References|GetDart%20Game%20Manager))
    (CallFunction|StopLineOfSight)
    (Variables|Interactions|SetPlayer%20In%20Range false)
    (CallFunction|HideStartingUI)
    (Variables|/Game/Player/BP_Player.BP_Player_C|SetCan%20Interact%20with%20Dart%20Board (Variables|References|GetPlayer%20Ref) false)
    (else
      (Variables|Interactions|SetPlayer%20In%20Range true)
      (CallFunction|StartLineOfSight))))

(event OnComponentEndOverlap(InteractCollision)
  (params (OverlappedComponent :type Primitive%20Component%20Object%20Reference) (OtherActor :type Actor%20Object%20Reference) (OtherComp :type Primitive%20Component%20Object%20Reference) (OtherBodyIndex :type Integer))
  ;[0 0 0] Interaction collision for starting line of sight and also only doing starting line of sight if darts game is not already active
  (Variables|Interactions|SetPlayer%20In%20Range false)
  (CallFunction|StopLineOfSight)
  (CallFunction|HideStartingUI))

(event Custom|Line%20of%20Sight%20Check
  (bind _player_ref (Variables|References|GetPlayer%20Ref))
  (bind _returnvalue (Pawn|GetControlRotation _player_ref :!class /Script/Engine.Pawn))
  (bind _outlocation (Actor|GetActorEyesViewPoint _player_ref))
  ;[0 0 0] Line of sight from player to dart board to see if the player is looking at the dart board and the game is not already active for setting UI hidden or shown
  (bind _returnvalue_2 (Class|KismetSystemLibrary|BoxTraceSingleforObjects _outlocation (+ (* (Math|Vector|GetForwardVector _returnvalue) 7.5e+02) _outlocation) "64.000000,256.000000,64.000000" _returnvalue (Utilities|Array|MakeArray "ObjectTypeQuery11") false 0 "None" false))
  (if _returnvalue_2
    (if (and (Variables|Interactions|GetPlayer%20In%20Range) (not (Variables|/Game/Mini_Games/Darts/BP_Dart_Game_Manager.BP_Dart_Game_Manager_C|GetDarts%20Game%20Active (Variables|References|GetDart%20Game%20Manager))))
      (Utilities|FlowControl|DoOnce false :!label _label
        (:Completed
          (Utilities|FlowControl|Sequence
            (:then_0
              (CallFunction|ShowStartingUI))
            (:then_1
              (goto _label_3 Reset)))))
      (else
        (Utilities|FlowControl|Sequence :!label _label_2
          (:then_0
            (goto _label Reset))
          (:then_1
            (Utilities|FlowControl|DoOnce false :!label _label_3
              (:Completed
                (CallFunction|HideStartingUI)))))))
    (else
      (goto _label_2))))

(event Custom|Start%20Line%20Of%20Sight
  ;[0 0 0] Start and stop line of sight functions
  (bind _returnvalue (Utilities|Time|SetTimerbyEvent (delegate Custom|Line%20of%20Sight%20Check) 0.05 true)))

(event Custom|Hide%20Scoreboard
  ;[0 0 0] Hide and show score board widget
  (bind _animation_length (Default|HideScoreboard (Variables|References|GetScoreboard%20Widget%20Ref)))
  (Utilities|FlowControl|Delay _animation_length)
  (Rendering|SetVisibility (Variables|Default|GetDart%20Scoreboard) false false))

(event Custom|Hide%20Winning%20Text
  ;[0 0 0] Events for hiding and showing the winning text and calling the update text function in the darts winner widget
  (Rendering|SetVisibility (Variables|Default|GetWinning%20Text%20Widget) false false))

(event Custom|Show%20Winning%20Text
  (params (Player%20Won? :type Boolean) (NPC%20Name :type Enum_NPC_Names%20Enum :default "NewEnumerator0"))
  ;[0 0 0] Events for hiding and showing the winning text and calling the update text function in the darts winner widget
  (Rendering|SetVisibility (Variables|Default|GetWinning%20Text%20Widget) true false)
  (Default|UpdateText (Variables|References|GetDarts%20Winner%20Text%20Ref) Player%20Won? NPC%20Name))

(event Custom|Stop%20Line%20of%20Sight
  ;[0 0 0] Start and stop line of sight functions
  (Utilities|Time|ClearandInvalidateTimerbyHandle (stale Custom|Start%20Line%20Of%20Sight _returnvalue))
  ;[0 0 0] Line of sight from player to dart board to see if the player is looking at the dart board and the game is not already active for setting UI hidden or shown
  (Utilities|FlowControl|DoOnce false) ; enters at Reset
)

(event Custom|Show%20Starting%20UI
  (bind _player_ref (Variables|References|GetPlayer%20Ref))
  ;[0 0 0] Setting UI visible and hidden and if the player can interact with the dart board
  (Rendering|SetVisibility (Variables|Default|GetStart%20Game%20Widget) true false)
  (Default|ShowStartButton (Variables|References|GetStart%20Game%20Widget%20Ref))
  (Default|ShowDifficulties (Variables|Default|GetDifficulty%20Selection%20Widget%20Ref))
  (Default|ShowModes (Variables|Default|GetDarts%20Mode%20Widget%20Ref))
  (Variables|/Game/Player/BP_Player.BP_Player_C|SetCan%20Interact%20with%20Dart%20Board _player_ref true)
  (Components|Activation|Activate (Variables|/Game/Player/BP_Player.BP_Player_C|GetWidget%20Interaction _player_ref) false))

(event Custom|Hide%20Starting%20UI
  (bind _player_ref (Variables|References|GetPlayer%20Ref))
  (bind _player_ref_2 (Variables|References|GetPlayer%20Ref))
  ;[0 0 0] Setting UI visible and hidden and if the player can interact with the dart board
  (Default|HideStartButton (Variables|References|GetStart%20Game%20Widget%20Ref))
  (Default|HideDifficulties (Variables|Default|GetDifficulty%20Selection%20Widget%20Ref))
  (Default|HideModes (Variables|Default|GetDarts%20Mode%20Widget%20Ref))
  (Variables|/Game/Player/BP_Player.BP_Player_C|SetCan%20Interact%20with%20Dart%20Board _player_ref false)
  (if (and (Utilities|Array|IsEmpty (Collision|GetOverlappingActors _player_ref_2 "/Game/NPCs/BP_NPC.BP_NPC_C" :!class /Script/Engine.Actor)) (Utilities|Array|IsEmpty (Collision|GetOverlappingActors _player_ref_2 "/Game/Misc_Mechanics/Jukebox/BP_Jukebox.BP_Jukebox_C" :!class /Script/Engine.Actor)))
    (Components|Activation|Deactivate (Variables|/Game/Player/BP_Player.BP_Player_C|GetWidget%20Interaction _player_ref)))
  (Utilities|FlowControl|Delay 0.25)
  (if (not (Variables|/Game/Player/BP_Player.BP_Player_C|GetCan%20Interact%20with%20Dart%20Board (Variables|References|GetPlayer%20Ref)))
    (Rendering|SetVisibility (Variables|Default|GetStart%20Game%20Widget) false false)))

(event Custom|Stop%20Player%20Aim%20Bar
  ;[0 0 0] Aim Sliders
  (if (== (Utilities|Array|Length (Variables|Scores|GetCurrent%20Player%20Aim%20Values)) 0)
    (Default|StopSlider (Variables|References|GetHorizontal%20Aim%20Widget%20Ref))
    (Utilities|Array|Add (Variables|Scores|GetCurrent%20Player%20Aim%20Values) (Variables|/Game/UI/Diegetic/Mini_Games/Darts/WBP_Darts_Aim_Bar.WBP_Darts_Aim_Bar_C|GetSlider%20Percent (Variables|References|GetHorizontal%20Aim%20Widget%20Ref)))
    (CallFunction|StartSliders)
    (else
      (Default|StopSlider (Variables|References|GetVertical%20Aim%20Widget%20Ref))
      (Utilities|Array|Add (Variables|Scores|GetCurrent%20Player%20Aim%20Values) (Variables|/Game/UI/Diegetic/Mini_Games/Darts/WBP_Darts_Aim_Bar.WBP_Darts_Aim_Bar_C|GetSlider%20Percent (Variables|References|GetVertical%20Aim%20Widget%20Ref)))
      (Default|PlayDart (Variables|References|GetDart%20Game%20Manager)))))

(event Custom|Reset%20Current%20Player%20Aim%20Values
  ;[0 0 0] Aim Sliders
  (Utilities|Array|Clear (Variables|Scores|GetCurrent%20Player%20Aim%20Values)))

(event Custom|Start%20Sliders
  ;[0 0 0] Aim Sliders
  (if (== (Utilities|Array|Length (Variables|Scores|GetCurrent%20Player%20Aim%20Values)) 0)
    (Default|SetupSlider (Variables|References|GetHorizontal%20Aim%20Widget%20Ref) (Variables|Default|GetSelected%20Difficulty))
    (Rendering|SetVisibility (Variables|Default|GetVertical%20Aim%20Slider) false false)
    (Rendering|SetVisibility (Variables|Default|GetHorizontal%20Aim%20Slider) true false)
    (Default|StartSlider (Variables|References|GetHorizontal%20Aim%20Widget%20Ref))
    (else
      (Default|SetupSlider (Variables|References|GetVertical%20Aim%20Widget%20Ref) (Variables|Default|GetSelected%20Difficulty))
      (Rendering|SetVisibility (Variables|Default|GetVertical%20Aim%20Slider) true false)
      (Default|StartSlider (Variables|References|GetVertical%20Aim%20Widget%20Ref)))))

(event Custom|Hide%20Both%20Sliders
  ;[0 0 0] Aim Sliders
  (Default|StopSlider (Variables|References|GetHorizontal%20Aim%20Widget%20Ref))
  (Default|StopSlider (Variables|References|GetVertical%20Aim%20Widget%20Ref))
  (Rendering|SetVisibility (Variables|Default|GetVertical%20Aim%20Slider) false false))

(event Custom|Show%20Scoreboard
  ;[0 0 0] Hide and show score board widget
  (Rendering|SetVisibility (Variables|Default|GetDart%20Scoreboard) true false)
  (Default|ShowScoreboard (Variables|References|GetScoreboard%20Widget%20Ref)))

(event EventBeginPlay
  ;[0 0 0] Setup for player ref and darts game manager ref
  (bind _returnvalue (Actor|GetActorOfClass "/Game/Player/BP_Player.BP_Player_C"))
  (Variables|References|SetPlayer%20Ref _returnvalue)
  (bind _returnvalue_2 (Actor|GetActorOfClass "/Game/Mini_Games/Darts/BP_Dart_Game_Manager.BP_Dart_Game_Manager_C"))
  (Variables|References|SetDart%20Game%20Manager _returnvalue_2)
  ;[0 0 0] Get widgets from the widget components and set references for later use
  (bind _aswbp_darts_aim_bar (Utilities|Casting|CastToWBP_Darts_Aim_Bar (UserInterface|GetWidget (Variables|Default|GetHorizontal%20Aim%20Slider))))
  (Variables|References|SetHorizontal%20Aim%20Widget%20Ref _aswbp_darts_aim_bar)
  (bind _aswbp_darts_aim_bar_2 (Utilities|Casting|CastToWBP_Darts_Aim_Bar (UserInterface|GetWidget (Variables|Default|GetVertical%20Aim%20Slider))))
  (Variables|References|SetVertical%20Aim%20Widget%20Ref _aswbp_darts_aim_bar_2)
  (bind _outactors (Actor|GetAllActorsOfClass "/Game/Mini_Games/Darts/Dart_Board/BP_Dart_Score_Point.BP_Dart_Score_Point_C"))
  (Variables|Scores|SetScore%20Point%20Actors _outactors)
  (bind _aswbp_darts_scoreboard (Utilities|Casting|CastToWBP_Darts_Scoreboard (UserInterface|GetWidget (Variables|Default|GetDart%20Scoreboard))))
  (Variables|References|SetScoreboard%20Widget%20Ref _aswbp_darts_scoreboard)
  (bind _aswbp_darts_winner (Utilities|Casting|CastToWBP_Darts_Winner (UserInterface|GetWidget (Variables|Default|GetWinning%20Text%20Widget))))
  (Variables|References|SetDarts%20Winner%20Text%20Ref _aswbp_darts_winner)
  (bind _aswbp_darts_start_game (Utilities|Casting|CastToWBP_Darts_Start_Game (UserInterface|GetWidget (Variables|Default|GetStart%20Game%20Widget))))
  (Variables|References|SetStart%20Game%20Widget%20Ref _aswbp_darts_start_game)
  (bind _aswbp_darts_difficulty_selection (Utilities|Casting|CastToWBP_Darts_Difficulty_Selection (UserInterface|GetWidget (Variables|Default|GetDifficulty%20Selection%20Widget))))
  (Variables|Default|SetDifficulty%20Selection%20Widget%20Ref _aswbp_darts_difficulty_selection)
  (bind _aswbp_darts_mode_selection (Utilities|Casting|CastToWBP_Darts_Mode_Selection (UserInterface|GetWidget (Variables|Default|GetDart%20Mode%20Selection%20Widget))))
  (Variables|Default|SetDarts%20Mode%20Widget%20Ref _aswbp_darts_mode_selection))

(fn ConstructionScript)