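; Dartboard actor for the darts mini-game that offers a start prompt and runs the player's aiming sliders.
; While the player is in range and no game is active, a looping timer box-traces from their view to toggle the prompt and interaction flag.
; Horizontal then vertical aim bars are stopped in turn, storing their percentages before BP_Dart_Game_Manager plays the dart.
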(event OnComponentBeginOverlap(InteractCollision)
  (params (OverlappedComponent :type Primitive%20Component%20Object%20Reference) (OtherActor :type Actor%20Object%20Reference) (OtherComp :type Primitive%20Component%20Object%20Reference) (OtherBodyIndex :type Integer) (bFromSweep :type Boolean) (SweepResult :type Hit%20Result%20Structure%20%28by%20ref%29))
  ;[0 0 0] Interaction collision for starting line of sight and also only doing starting line of sight if darts game is not already active
  (if (Variables|/Game/Mini_Games/Darts/BP_Dart_Game_Manager.BP_Dart_Game_Manager_C|GetDarts%20Game%20Active (Variables|Default|GetDart%20Game%20Manager))
    (CallFunction|StopLineOfSight)
    (Variables|Default|SetPlayer%20In%20Range false)
    (CallFunction|HideUI)
    (Variables|/Game/Player/BP_Player.BP_Player_C|SetCan%20Interact%20with%20Dart%20Board (Variables|Default|GetPlayer%20Ref) false)
    (else
      (Variables|Default|SetPlayer%20In%20Range true)
      (CallFunction|StartLineOfSight))))

(event OnComponentEndOverlap(InteractCollision)
  (params (OverlappedComponent :type Primitive%20Component%20Object%20Reference) (OtherActor :type Actor%20Object%20Reference) (OtherComp :type Primitive%20Component%20Object%20Reference) (OtherBodyIndex :type Integer))
  ;[0 0 0] Interaction collision for starting line of sight and also only doing starting line of sight if darts game is not already active
  (Variables|Default|SetPlayer%20In%20Range false)
  (CallFunction|StopLineOfSight)
  (CallFunction|HideUI))

(event Custom|Line%20of%20Sight%20Check
  (bind _player_ref (Variables|Default|GetPlayer%20Ref))
  (bind _returnvalue (Pawn|GetControlRotation _player_ref :!class /Script/Engine.Pawn))
  (bind _outlocation (Actor|GetActorEyesViewPoint _player_ref))
  ;[0 0 0] Line of sight from player to dart board to see if the player is looking at the dart board and the game is not already active for setting UI hidden or shown
  (bind _returnvalue_2 (Class|KismetSystemLibrary|BoxTraceSingleforObjects _outlocation (+ (* (Math|Vector|GetForwardVector _returnvalue) 5e+02) _outlocation) "16.000000,16.000000,16.000000" _returnvalue (Utilities|Array|MakeArray "ObjectTypeQuery11") false 0 "ForOneFrame" false))
  (if _returnvalue_2
    (if (and (Variables|Default|GetPlayer%20In%20Range) (not (Variables|/Game/Mini_Games/Darts/BP_Dart_Game_Manager.BP_Dart_Game_Manager_C|GetDarts%20Game%20Active (Variables|Default|GetDart%20Game%20Manager))))
      (Utilities|FlowControl|DoOnce false :!label _label
        (:Completed
          (Utilities|FlowControl|Sequence
            (:then_0
              (CallFunction|ShowUI))
            (:then_1
              (goto _label_3 Reset)))))
      (else
        (Utilities|FlowControl|Sequence :!label _label_2
          (:then_0
            (goto _label Reset))
          (:then_1
            (Utilities|FlowControl|DoOnce false :!label _label_3
              (:Completed
                (CallFunction|HideUI)))))))
    (else
      (goto _label_2))))

(event Custom|Start%20Line%20Of%20Sight
  ;[0 0 0] Start and stop line of sight functions
  (bind _returnvalue (Utilities|Time|SetTimerbyEvent (delegate Custom|Line%20of%20Sight%20Check) 0.05 true)))

(event Custom|Stop%20Line%20of%20Sight
  ;[0 0 0] Start and stop line of sight functions
  (Utilities|Time|ClearandInvalidateTimerbyHandle (stale Custom|Start%20Line%20Of%20Sight _returnvalue)))

(event Custom|Show%20UI
  ;[0 0 0] Setting UI visible and hidden and if the player can interact with the dart board
  (Rendering|SetVisibility (Variables|Default|GetStart%20Game%20Widget) true false)
  (Variables|/Game/Player/BP_Player.BP_Player_C|SetCan%20Interact%20with%20Dart%20Board (Variables|Default|GetPlayer%20Ref) true))

(event Custom|Hide%20UI
  ;[0 0 0] Setting UI visible and hidden and if the player can interact with the dart board
  (Rendering|SetVisibility (Variables|Default|GetStart%20Game%20Widget) false false)
  (Variables|/Game/Player/BP_Player.BP_Player_C|SetCan%20Interact%20with%20Dart%20Board (Variables|Default|GetPlayer%20Ref) false))

(event Custom|Stop%20Player%20Aim%20Bar
  (if (== (Utilities|Array|Length (Variables|Default|GetCurrent%20Player%20Aim%20Values)) 0)
    (Default|StopSlider (Variables|Default|GetHoriontal%20Aim%20Widget%20Ref))
    (Utilities|Array|Add (Variables|Default|GetCurrent%20Player%20Aim%20Values) (Variables|/Game/UI/Diegetic/Mini_Games/WBP_Darts_Aim_Bar.WBP_Darts_Aim_Bar_C|GetSlider%20Percent (Variables|Default|GetHoriontal%20Aim%20Widget%20Ref)))
    (CallFunction|StartSliders)
    (else
      (Default|StopSlider (Variables|Default|GetVertical%20Aim%20Widget%20Ref))
      (Utilities|Array|Add (Variables|Default|GetCurrent%20Player%20Aim%20Values) (Variables|/Game/UI/Diegetic/Mini_Games/WBP_Darts_Aim_Bar.WBP_Darts_Aim_Bar_C|GetSlider%20Percent (Variables|Default|GetVertical%20Aim%20Widget%20Ref)))
      (Default|PlayDart (Variables|Default|GetDart%20Game%20Manager)))))

(event Custom|Reset%20Current%20Player%20Aim%20Values
  (Utilities|Array|Clear (Variables|Default|GetCurrent%20Player%20Aim%20Values)))

(event Custom|Start%20Sliders
  (if (== (Utilities|Array|Length (Variables|Default|GetCurrent%20Player%20Aim%20Values)) 0)
    (Default|SetupSlider (Variables|Default|GetHoriontal%20Aim%20Widget%20Ref))
    (Rendering|SetVisibility (Variables|Default|GetVertical%20Aim%20Slider) false false)
    (Rendering|SetVisibility (Variables|Default|GetHorizontal%20Aim%20Slider) true false)
    (Default|StartSlider (Variables|Default|GetHoriontal%20Aim%20Widget%20Ref))
    (else
      (Default|SetupSlider (Variables|Default|GetVertical%20Aim%20Widget%20Ref))
      (Rendering|SetVisibility (Variables|Default|GetVertical%20Aim%20Slider) true false)
      (Default|StartSlider (Variables|Default|GetVertical%20Aim%20Widget%20Ref)))))

(event Custom|Hide%20Both%20Sliders
  (Default|StopSlider (Variables|Default|GetHoriontal%20Aim%20Widget%20Ref))
  (Default|StopSlider (Variables|Default|GetVertical%20Aim%20Widget%20Ref))
  (Rendering|SetVisibility (Variables|Default|GetVertical%20Aim%20Slider) false false))

(event EventBeginPlay
  ;[0 0 0] Setup for player ref and darts game manager ref
  (bind _returnvalue (Actor|GetActorOfClass "/Game/Player/BP_Player.BP_Player_C"))
  (Variables|Default|SetPlayer%20Ref _returnvalue)
  (bind _returnvalue_2 (Actor|GetActorOfClass "/Game/Mini_Games/Darts/BP_Dart_Game_Manager.BP_Dart_Game_Manager_C"))
  (Variables|Default|SetDart%20Game%20Manager _returnvalue_2)
  ;[0 0 0] Get widgets from the widget components and set references for later use
  (bind _aswbp_darts_aim_bar (Utilities|Casting|CastToWBP_Darts_Aim_Bar (UserInterface|GetWidget (Variables|Default|GetHorizontal%20Aim%20Slider))))
  (Variables|Default|SetHoriontal%20Aim%20Widget%20Ref _aswbp_darts_aim_bar)
  (bind _aswbp_darts_aim_bar_2 (Utilities|Casting|CastToWBP_Darts_Aim_Bar (UserInterface|GetWidget (Variables|Default|GetVertical%20Aim%20Slider))))
  (Variables|Default|SetVertical%20Aim%20Widget%20Ref _aswbp_darts_aim_bar_2))

(fn ConstructionScript)