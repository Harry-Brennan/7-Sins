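; Shared turn manager that tracks whose turn it is in the card games and 1v1 mini games.
; Setup functions fill the player list, and StartFirstTurn opens I Doubt It with the Ace of Spades holder or Rat Screw at random.
; Turns advance through a wrapping, reversible index and notify characters via TakeTurnMessage.
; A widget indicator glides between players on a timeline, attaches to the current one, then bounces.
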(event Custom|Update%20Current%20Turn%20Indicator
  (params (Previously%20Played%20Player :type Actor%20Object%20Reference))
  (bind _playing_characters (Variables|TurnTaking|GetPlaying%20Characters))
  (bind _current_character_turn_index_ (Variables|TurnTaking|GetCurrent%20Character%20Turn%20Index%20))
  (bind _output (Utilities|Array|Get(acopy) _playing_characters _current_character_turn_index_))
  (Transformation|DetachFromComponent (Variables|Default|GetCurrent%20Turn%20Indicator) "KeepWorld" "KeepWorld" "KeepWorld" true)
  (Rendering|SetVisibility (Variables|Default|GetCurrent%20Turn%20Indicator) true false)
  (bind _alpha (Timeline|Turn%20Indicator%20Timeline PlayFromStart)
    (:Update
      (Transformation|SetWorldLocationAndRotation (Variables|Default|GetCurrent%20Turn%20Indicator) (Math|Vector|Lerp(Vector) (+ (Transformation|GetActorLocation Previously%20Played%20Player) "0.000000,0.000000,180.000000") (+ (Transformation|GetActorLocation _output) "0.000000,0.000000,180.000000") _alpha) (Math|Rotator|Lerp(Rotator) (Transformation|GetActorRotation Previously%20Played%20Player) (Transformation|GetActorRotation _output) _alpha true) false false))
    (:Finished
      (Transformation|AttachComponentToComponent (Variables|Default|GetCurrent%20Turn%20Indicator) (Variables|/Script/Engine.Actor|GetRootComponent (Utilities|Array|Get(acopy) (Variables|TurnTaking|GetPlaying%20Characters) (Variables|TurnTaking|GetCurrent%20Character%20Turn%20Index%20))) "None" "KeepWorld" "KeepWorld" "KeepWorld" true)
      (CallFunction|PlayTurnIndicatorBounceAnimation))))

(event Custom|Play%20Turn%20Indicator%20Bounce%20Animation
  (Variables|Widget|SetBounce%20Start%20Location (Transformation|GetWorldLocation (Variables|Default|GetCurrent%20Turn%20Indicator)))
  (bind _alpha (Timeline|Turn%20Indicator%20Bounce%20Animation PlayFromStart)
    (:Update
      (Transformation|SetWorldLocation (Variables|Default|GetCurrent%20Turn%20Indicator) (Math|Vector|Lerp(Vector) (Variables|Widget|GetBounce%20Start%20Location) (- (Variables|Widget|GetBounce%20Start%20Location) (Math|Vector|MakeVector 0.0 0.0 (Variables|Widget|GetBounce%20Movement%20Amount))) _alpha) false false))))

(event EventBeginPlay
  (bind _returnvalue (Actor|GetActorOfClass "/Game/Shared_Game_Mechanics/Cards/BP_Card_Dealer.BP_Card_Dealer_C"))
  (Variables|References|SetCard%20Dealer%20Reference _returnvalue)
  (bind _returnvalue_2 (Actor|GetActorOfClass "/Game/Main_Game_Managers/I_Doubt_It/BP_I_Doubt_It_Game_Manager.BP_I_Doubt_It_Game_Manager_C"))
  (Variables|References|SetI%20Doubt%20It%20Game%20Manager _returnvalue_2)
  (bind _returnvalue_3 (AddComponent|AddWidgetComponent false))
  (Rendering|SetVisibility _returnvalue_3 false false)
  (Variables|Default|SetCurrent%20Turn%20Indicator _returnvalue_3))

(fn ConstructionScript)

(fn SetupMainGame
  (params (Main%20Game%20Name :type Enum_Main_Game_Names%20Enum :default "Enum_Main_Game_Names_MAX") (Playing%20Characters%20Passed :type Array%20of%20Actor%20Object%20References))
  ;[1 1 1] Pass the main game name that is being played as well as the playing opponents
  ;[1 1 1] Clear the playing characters array since this is a new game being played
  (Utilities|Array|Clear (Variables|TurnTaking|GetPlaying%20Characters))
  ;[1 1 1] Set the current character index turn (the current character in the array whose turn it is) to be 0 since this is a new game
  (Variables|TurnTaking|SetCurrent%20Character%20Turn%20Index%20 0)
  ;[1 1 1] Switch based on the game being played
  (switch Utilities|FlowControl|Switch|SwitchonEnum_Main_Game_Names Main%20Game%20Name
    (:NewEnumerator0
      ;[1 1 1] I doubt it and auction are multiple opponent games so the method is multi whereas rat screw is a 1v1 game so the method is 1v1
      (Variables|TurnTaking|SetCurrent%20Turn%20Taking%20Methods "NewEnumerator1" :!label _label))
    (:NewEnumerator1
      (goto _label))
    (:NewEnumerator2
      (Variables|TurnTaking|SetCurrent%20Turn%20Taking%20Methods "NewEnumerator0")))
  ;[1 1 1] Set playing characters to be the passed playing characters
  (Variables|TurnTaking|SetPlaying%20Characters Playing%20Characters%20Passed))

(fn SetupMiniGame
  (params (NPC%20Opponent :type Actor%20Object%20Reference))
  ;[1 1 1] Pass the NPC opponent that is playing the game
  ;[1 1 1] Clear the playing characters array since this is a new game
  (Utilities|Array|Clear (Variables|TurnTaking|GetPlaying%20Characters))
  ;[1 1 1] Set the current character turn index to be 0 since this is a new game
  (Variables|TurnTaking|SetCurrent%20Character%20Turn%20Index%20 0)
  ;[1 1 1] All mini games are 1v1
  (Variables|TurnTaking|SetCurrent%20Turn%20Taking%20Methods "NewEnumerator0")
  ;[1 1 1] Get the player and add them to the playing characters array
  (bind _returnvalue (Actor|GetActorOfClass "/Game/Player/BP_Player.BP_Player_C"))
  (Utilities|Array|Add (Variables|TurnTaking|GetPlaying%20Characters) _returnvalue)
  ;[1 1 1] Add the NPC opponent to the playing characters array
  (Utilities|Array|Add (Variables|TurnTaking|GetPlaying%20Characters) NPC%20Opponent))

(fn StartFirstTurn
  (params (Game%20Name :type Enum_Main_Game_Names%20Enum :default "NewEnumerator0"))
  (bind _playing_characters (Variables|TurnTaking|GetPlaying%20Characters))
  (switch Utilities|FlowControl|Switch|SwitchonEnum_Main_Game_Names Game%20Name
    (:NewEnumerator0
      ;[1 1 1] Find the ace of spaedes and store the reference to the card that is the ace of spades also store a reference to the current player in the loop
      (bind (_array_element _array_index) (Utilities|Array|ForEachLoopwithBreak (Variables|TurnTaking|GetPlaying%20Characters) :!label _label)
        (:LoopBody
          (LocalVariables|SetIDI%20Counter _array_index)
          (LocalVariables|SetIDI%20Current%20Player _array_element)
          (bind _array_element_2 (Utilities|Array|ForEachLoopwithBreak (Variables|/Game/Shared_Game_Mechanics/BPC_CurrentHand.BPC_CurrentHand_C|GetCurrent%20Hand (Actor|GetComponentbyClass _array_element "/Game/Shared_Game_Mechanics/BPC_CurrentHand.BPC_CurrentHand_C")) :!label _label_2)
            (:LoopBody
              (bind _card_info (Default|GetCardInfo _array_element_2))
              (if (and (Utilities|Enum|Equal(Enum) (.CardName (Utilities|Struct|BreakStruct_Card _card_info)) "NewEnumerator0") (Utilities|Enum|Equal(Enum) (.Suit (Utilities|Struct|BreakStruct_Card _card_info)) "NewEnumerator0"))
                (LocalVariables|SetIDI%20Ace%20Of%20Spades%20Card%20Ref _array_element_2)
                (Utilities|FlowControl|Sequence
                  (:then_0
                    (goto _label_2 Break))
                  (:then_1
                    (goto _label Break)))))))
        (:Completed
          ;[1 1 1] Call end player turn function in the IDI game manager and pass the player with the ace of spades and the ace of spades card to this and then set the current character turn index to be the character that just had the ace of spades
          (Development|PrintString (Utilities|String|Append (Utilities|GetDisplayName (LocalVariables|GetIDI%20Current%20Player)) " HAS JUST PLAYED THE ACE OF SPADES") true true "(R=0.767572,G=0.153618,B=1.000000,A=1.000000)" 1e+02)
          (Development|PrintString (Utilities|String|ToString(Integer) (LocalVariables|GetIDI%20Counter)) true true "(R=1.000000,G=0.000000,B=0.067183,A=1.000000)" 1e+02)
          (Variables|TurnTaking|SetCurrent%20Character%20Turn%20Index%20 (LocalVariables|GetIDI%20Counter))
          (Widget|SetupCurrentTurnIndicatorStartingLocandRot)
          (Default|EndPlayerTurn (Variables|References|GetI%20Doubt%20It%20Game%20Manager) (LocalVariables|GetIDI%20Current%20Player) (Utilities|Array|MakeArray (LocalVariables|GetIDI%20Ace%20Of%20Spades%20Card%20Ref))))))
    (:NewEnumerator2
      (if (Math|Random|RandomBoolwithWeight 0.5)
        (Variables|TurnTaking|SetCurrent%20Character%20Turn%20Index%20 0)
        (Class|BPIPlayingCharacter|TakeTurn(Message) (Utilities|Array|Get(acopy) _playing_characters))
        (else
          (Variables|TurnTaking|SetCurrent%20Character%20Turn%20Index%20 1)
          (Class|BPIPlayingCharacter|TakeTurn(Message) (Utilities|Array|Get(acopy) _playing_characters 1))))
      (Widget|SetupCurrentTurnIndicatorStartingLocandRot))))

(fn NextPlayerTurn
  ;[0 0 0] If this new incremented index is greater than the last index in the playing characters array then loop back to the start by setting it ot 0 and if not then just set it to be the incremented version - using macro version now
  (Variables|TurnTaking|SetCurrent%20Character%20Turn%20Index%20 (GetIndexes|GetNextCharacterIndex))
  ;[0 0 0] Updating the visibility of the current turn widget for the new current player
  (CallFunction|UpdateCurrentTurnIndicator (Utilities|Array|Get(acopy) (Variables|TurnTaking|GetPlaying%20Characters) (GetIndexes|GetPreviousCharacterIndex)))
  ;[0 0 0] Debug Message
  (Development|PrintString (Utilities|String|Append "CURRENT TURN : " (Utilities|GetDisplayName (Utilities|Array|Get(acopy) (Variables|TurnTaking|GetPlaying%20Characters) (Variables|TurnTaking|GetCurrent%20Character%20Turn%20Index%20)))) true true "(R=0.801141,G=1.000000,B=0.000000,A=1.000000)" 1e+02)
  ;[0 0 0] Call the take turn function in the corresponding character whose turn it is
  (Class|BPIPlayingCharacter|TakeTurn(Message) (Utilities|Array|Get(acopy) (Variables|TurnTaking|GetPlaying%20Characters) (Variables|TurnTaking|GetCurrent%20Character%20Turn%20Index%20))))

(fn SamePlayerTurn
  (Class|BPIPlayingCharacter|TakeTurn(Message) (Utilities|Array|Get(acopy) (Variables|TurnTaking|GetPlaying%20Characters) (Variables|TurnTaking|GetCurrent%20Character%20Turn%20Index%20))))

(fn SwitchTurnDirection
  (Variables|TurnTaking|SetDirection (not (Variables|TurnTaking|GetDirection))))

(fn GetNextCharacterIndex
  (bind _playing_characters (Variables|TurnTaking|GetPlaying%20Characters))
  (bind _current_character_turn_index_ (Variables|TurnTaking|GetCurrent%20Character%20Turn%20Index%20))
  (bind _current_character_turn_index__2 (Variables|TurnTaking|GetCurrent%20Character%20Turn%20Index%20))
  (bind _returnvalue (Utilities|Array|LastIndex _playing_characters))
  (bind _returnvalue_2 (+ _current_character_turn_index_ 1))
  (bind _returnvalue_3 (- _current_character_turn_index__2 1))
  (return (Math|Integer|SelectInt (Math|Integer|SelectInt 0 _returnvalue_2 (> _returnvalue_2 _returnvalue)) (Math|Integer|SelectInt _returnvalue _returnvalue_3 (< _returnvalue_3 0)) (Variables|TurnTaking|GetDirection))))

(fn GetPreviousCharacterIndex
  (bind _playing_characters (Variables|TurnTaking|GetPlaying%20Characters))
  (bind _current_character_turn_index_ (Variables|TurnTaking|GetCurrent%20Character%20Turn%20Index%20))
  (bind _current_character_turn_index__2 (Variables|TurnTaking|GetCurrent%20Character%20Turn%20Index%20))
  (bind _returnvalue (Utilities|Array|LastIndex _playing_characters))
  (bind _returnvalue_2 (+ _current_character_turn_index_ 1))
  (bind _returnvalue_3 (- _current_character_turn_index__2 1))
  (return (Math|Integer|SelectInt (Math|Integer|SelectInt _returnvalue _returnvalue_3 (< _returnvalue_3 0)) (Math|Integer|SelectInt 0 _returnvalue_2 (> _returnvalue_2 _returnvalue)) (Variables|TurnTaking|GetDirection))))

(fn SetupCurrentTurnIndicatorStartingLocandRot
  (bind _playing_characters (Variables|TurnTaking|GetPlaying%20Characters))
  (bind _current_character_turn_index_ (Variables|TurnTaking|GetCurrent%20Character%20Turn%20Index%20))
  (bind _output (Utilities|Array|Get(acopy) _playing_characters _current_character_turn_index_))
  (Rendering|SetVisibility (Variables|Default|GetCurrent%20Turn%20Indicator) true false)
  (Transformation|SetWorldLocationAndRotation (Variables|Default|GetCurrent%20Turn%20Indicator) (+ (Transformation|GetActorLocation _output) "0.000000,0.000000,180.000000") (Transformation|GetActorRotation _output) false false))