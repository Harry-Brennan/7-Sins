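; BP_Rat_Screw_Game_Manager sets up a Rat Screw card game, starting two seconds after BeginPlay.
; BeginGame stores player references, spawns player, opponent and shared BP_CardPile actors, then has the level's BP_Card_Dealer set up, shuffle and deal.
; DealToPlayers looks unfinished: its length check picks the receiving pile, always adds the first card, and removes it only on the opponent branch.
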(event EventBeginPlay
  (bind _returnvalue (Actor|GetActorOfClass "/Game/Shared_Game_Mechanics/Cards/BP_Card_Dealer.BP_Card_Dealer_C"))
  (Variables|Default|SetCard%20Dealer%20Reference _returnvalue)
  (Utilities|FlowControl|Delay 2.0)
  (CallFunction|BeginGame (Game|GetPlayerCharacter 0)))

(event Collision|EventActorBeginOverlap
  (params (OtherActor :type Actor%20Object%20Reference)))

(event EventTick
  (params (DeltaSeconds :type Float%20%28single-precision%29)))

(event Input|KeyboardEvents|DebugKeyT
  (params (Key :type Key%20Structure :default "None") (ActionValue :type Input%20Action%20Value%20Structure)))

(fn ConstructionScript)

(fn BeginGame
  (params (Playing%20Character :type Actor%20Object%20Reference) (Player :type Actor%20Object%20Reference))
  (bind _card_dealer_reference (Variables|Default|GetCard%20Dealer%20Reference))
  (Variables|Default|SetOpponent%20Reference Playing%20Character)
  (Variables|Default|SetPlayer%20Reference Player)
  (bind _returnvalue (Game|SpawnActorfromClass "/Game/Shared_Game_Mechanics/Cards/BP_CardPile.BP_CardPile_C" (Math|Transform|MakeTransform "0, 0, 0" "0, 0, 0" "1.000000,1.000000,1.000000") "Undefined" "MultiplyWithRoot" 0 0))
  (Variables|Default|SetPlayerCardPIle _returnvalue)
  (bind _returnvalue_2 (Game|SpawnActorfromClass "/Game/Shared_Game_Mechanics/Cards/BP_CardPile.BP_CardPile_C" (Math|Transform|MakeTransform "0, 0, 0" "0, 0, 0" "1.000000,1.000000,1.000000") "Undefined" "MultiplyWithRoot" 0 0))
  (Variables|Default|SetOpponentCardPile _returnvalue_2)
  (bind _returnvalue_3 (Game|SpawnActorfromClass "/Game/Shared_Game_Mechanics/Cards/BP_CardPile.BP_CardPile_C" (Math|Transform|MakeTransform "0, 0, 0" "0, 0, 0" "1.000000,1.000000,1.000000") "Undefined" "MultiplyWithRoot" 0 0))
  (Variables|Default|SetSharedCardPile _returnvalue_3)
  (Default|SetupCards _card_dealer_reference "NewEnumerator2")
  (Default|ShuffleCards _card_dealer_reference)
  (Default|DealCards _card_dealer_reference "NewEnumerator2"))

(fn DealtoPlayers
  (params (Cards :type Array%20of%20BP%20Card%20Object%20References))
  (bind _output (Utilities|Array|Get(acopy) Cards))
  (Utilities|Array|ForEachLoopwithBreak Cards
    (:LoopBody
      (if (== 0 (- (/ (Utilities|Array|Length Cards) 2) 1))
        (Utilities|Array|Add (Variables|/Game/Shared_Game_Mechanics/Cards/BP_CardPile.BP_CardPile_C|GetCardsInPile (Variables|Default|GetOpponentCardPile)) _output)
        (Utilities|Array|RemoveItem Cards _output)
        (else
          (Utilities|Array|Add (Variables|/Game/Shared_Game_Mechanics/Cards/BP_CardPile.BP_CardPile_C|GetCardsInPile (Variables|Default|GetPlayerCardPIle)) _output))))))