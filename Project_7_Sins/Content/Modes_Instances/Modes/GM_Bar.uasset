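; GM_Bar is the bar's game mode, tracking which minigame is active: I Doubt It, Auction, Rat Screw, Pool or Darts.
; BeginPlay caches manager references and creates per-game prompt widgets and the pause menu.
; Switching games swaps prompts and Enhanced Input mapping contexts via Selects on the current game.
; It also toggles the pause menu, routes pause/resume or delayed starts to some managers, and stores sound-class volumes.
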(event EventBeginPlay
  (bind _returnvalue (Actor|GetActorOfClass "/Game/Main_Game_Managers/Auction/BP_Auction_Game_Manager.BP_Auction_Game_Manager_C"))
  (Variables|References|SetAuction%20GM _returnvalue)
  (bind _returnvalue_2 (Actor|GetActorOfClass "/Game/Main_Game_Managers/I_Doubt_It/BP_I_Doubt_It_Game_Manager.BP_I_Doubt_It_Game_Manager_C"))
  (Variables|References|SetIDI%20GM _returnvalue_2)
  (bind _returnvalue_3 (Actor|GetActorOfClass "/Game/Main_Game_Managers/Rat_Screw/BP_Rat_Screw_Game_Manager.BP_Rat_Screw_Game_Manager_C"))
  (Variables|References|SetRat%20Screw%20GM _returnvalue_3)
  (Utilities|SetupPromptWidgets
    (:Out
      (CallFunction|SetCurrentPlayingGame "NewEnumerator5")
      (bind _returnvalue_4 (UserInterface|CreateWidget "/Game/UI/Non_Diegetic/Pause/WBP_Pause_Menu.WBP_Pause_Menu_C"))
      (Variables|References|SetPause%20Screen%20Widget _returnvalue_4)
      (bind _returnvalue_5 (Actor|GetActorOfClass "/Game/Mini_Games/Darts/BP_Dart_Game_Manager.BP_Dart_Game_Manager_C"))
      (Variables|References|SetDart%20Game%20Manager%20Ref _returnvalue_5))))

(fn ConstructionScript)

(fn SetCurrentPlayingGame
  (params (Current%20Game :type Enum_All_Game_Names%20Enum :default "NewEnumerator0"))
  ;[0 0 0] Remove the button prompt for the active game and set the current playing game after this to be the passed current game and then add the button prompts for this new current game to the viewport
  (Widget|RemovefromParent (Utilities|Select :Index (Variables|CurrentGame|GetCurrent%20Playing%20Game) :NewEnumerator0 (Variables|ButtonPromptWidgets|GetIDI%20Button%20Prompt%20Widget) :NewEnumerator1 (Variables|ButtonPromptWidgets|GetAuction%20Button%20Prompt%20Widget) :NewEnumerator2 (Variables|ButtonPromptWidgets|GetRat%20Screw%20Button%20Prompt%20Widget) :NewEnumerator3 (Variables|ButtonPromptWidgets|GetPool%20Button%20Prompt%20Widget) :NewEnumerator4 (Variables|ButtonPromptWidgets|GetDarts%20Button%20Prompt%20Widget) :NewEnumerator5 (Variables|ButtonPromptWidgets|GetBar%20Button%20Prompt%20Widget)))
  (Variables|CurrentGame|SetCurrent%20Playing%20Game Current%20Game)
  (UserInterface|Viewport|AddtoViewport (Utilities|Select :Index (Variables|CurrentGame|GetCurrent%20Playing%20Game) :NewEnumerator0 (Variables|ButtonPromptWidgets|GetIDI%20Button%20Prompt%20Widget) :NewEnumerator1 (Variables|ButtonPromptWidgets|GetAuction%20Button%20Prompt%20Widget) :NewEnumerator2 (Variables|ButtonPromptWidgets|GetRat%20Screw%20Button%20Prompt%20Widget) :NewEnumerator3 (Variables|ButtonPromptWidgets|GetPool%20Button%20Prompt%20Widget) :NewEnumerator4 (Variables|ButtonPromptWidgets|GetDarts%20Button%20Prompt%20Widget) :NewEnumerator5 (Variables|ButtonPromptWidgets|GetBar%20Button%20Prompt%20Widget)) 0)
  ;[0 0 0] Set game active if we are playing any game that isn't none
  (Variables|CurrentGame|SetGame%20Active (not (Utilities|Enum|Equal(Enum) (Variables|CurrentGame|GetCurrent%20Playing%20Game) "NewEnumerator5")))
  ;[0 0 0] Remove the bar mapping context and add the corresponding input mapping for the new current game
  (bind _returnvalue (Actor|GetActorOfClass "/Game/Player/BP_Player.BP_Player_C"))
  (bind _asplayer_controller (Utilities|Casting|CastToPlayerController (Pawn|GetController _returnvalue)))
  (Utilities|IsValid (PlayerController|LocalPlayerSubsystems|GetEnhancedInputLocalPlayerSubsystem _asplayer_controller)
    (:Is%20Valid
      (Input|RemoveMappingContext (PlayerController|LocalPlayerSubsystems|GetEnhancedInputLocalPlayerSubsystem _asplayer_controller) "/Game/Player/Input/IMC/IMC_Bar.IMC_Bar" "(bIgnoreAllPressedKeysUntilRelease=True,bForceImmediately=False,bNotifyUserSettings=False)")
      (Input|AddMappingContext (PlayerController|LocalPlayerSubsystems|GetEnhancedInputLocalPlayerSubsystem _asplayer_controller) (Utilities|Select :Index Current%20Game :NewEnumerator0 "/Game/Player/Input/IMC/IMC_I_Doubt_It.IMC_I_Doubt_It" :NewEnumerator1 "/Game/Player/Input/IMC/IMC_Auction.IMC_Auction" :NewEnumerator2 "/Game/Player/Input/IMC/IMC_Rat_Screw.IMC_Rat_Screw" :NewEnumerator3 "/Game/Player/Input/IMC/IMC_Pool.IMC_Pool" :NewEnumerator4 "/Game/Player/Input/IMC/IMC_Darts.IMC_Darts" :NewEnumerator5 "/Game/Player/Input/IMC/IMC_Bar.IMC_Bar") 0 "(bIgnoreAllPressedKeysUntilRelease=True,bForceImmediately=False,bNotifyUserSettings=False)"))))

(fn DEBUGLeaveCurrentGame
  (Variables|CurrentGame|SetGame%20Active false)
  (bind _returnvalue (Actor|GetActorOfClass "/Game/Player/BP_Player.BP_Player_C"))
  (bind _asplayer_controller (Utilities|Casting|CastToPlayerController (Pawn|GetController _returnvalue)))
  (Utilities|IsValid (PlayerController|LocalPlayerSubsystems|GetEnhancedInputLocalPlayerSubsystem _asplayer_controller)
    (:Is%20Valid
      (Input|RemoveMappingContext (PlayerController|LocalPlayerSubsystems|GetEnhancedInputLocalPlayerSubsystem _asplayer_controller) (Utilities|Select :Index (Variables|CurrentGame|GetCurrent%20Playing%20Game) :NewEnumerator0 "/Game/Player/Input/IMC/IMC_I_Doubt_It.IMC_I_Doubt_It" :NewEnumerator1 "/Game/Player/Input/IMC/IMC_Auction.IMC_Auction" :NewEnumerator2 "/Game/Player/Input/IMC/IMC_Rat_Screw.IMC_Rat_Screw" :NewEnumerator3 "/Game/Player/Input/IMC/IMC_Pool.IMC_Pool" :NewEnumerator4 "/Game/Player/Input/IMC/IMC_Darts.IMC_Darts" :NewEnumerator5 "/Game/Player/Input/IMC/IMC_Bar.IMC_Bar") "(bIgnoreAllPressedKeysUntilRelease=True,bForceImmediately=False,bNotifyUserSettings=False)")
      (Input|AddMappingContext (PlayerController|LocalPlayerSubsystems|GetEnhancedInputLocalPlayerSubsystem _asplayer_controller) "/Game/Player/Input/IMC/IMC_Bar.IMC_Bar" 0 "(bIgnoreAllPressedKeysUntilRelease=True,bForceImmediately=False,bNotifyUserSettings=False)")
      (Widget|RemovefromParent (Utilities|Select :Index (Variables|CurrentGame|GetCurrent%20Playing%20Game) :NewEnumerator0 (Variables|ButtonPromptWidgets|GetIDI%20Button%20Prompt%20Widget) :NewEnumerator1 (Variables|ButtonPromptWidgets|GetAuction%20Button%20Prompt%20Widget) :NewEnumerator2 (Variables|ButtonPromptWidgets|GetRat%20Screw%20Button%20Prompt%20Widget) :NewEnumerator3 (Variables|ButtonPromptWidgets|GetPool%20Button%20Prompt%20Widget) :NewEnumerator4 (Variables|ButtonPromptWidgets|GetDarts%20Button%20Prompt%20Widget) :NewEnumerator5 (Variables|ButtonPromptWidgets|GetBar%20Button%20Prompt%20Widget)))
      (Variables|CurrentGame|SetCurrent%20Playing%20Game "NewEnumerator5")
      (UserInterface|Viewport|AddtoViewport (Variables|ButtonPromptWidgets|GetBar%20Button%20Prompt%20Widget) 0))))

(fn PausePlayingGame
  ;[0 0 0] Call specific pause functions in the game manager corresponding to the current game
  (switch Utilities|FlowControl|Switch|SwitchonEnum_All_Game_Names (Variables|CurrentGame|GetCurrent%20Playing%20Game)
    (:NewEnumerator0
      (Default|PausePlayerTurn (Variables|References|GetIDI%20GM)))
    (:NewEnumerator1
      (Default|PauseRound (Variables|References|GetAuction%20GM)))))

(fn UnpausePlayingGame
  ;[0 0 0] Unpause the game or start the game if the current round index is less than 1 for the corresponding game for the current game
  (switch Utilities|FlowControl|Switch|SwitchonEnum_All_Game_Names (Variables|CurrentGame|GetCurrent%20Playing%20Game)
    (:NewEnumerator0
      (if (> (Variables|/Game/Main_Game_Managers/I_Doubt_It/BP_I_Doubt_It_Game_Manager.BP_I_Doubt_It_Game_Manager_C|GetCurrent%20Round%20Index (Variables|References|GetIDI%20GM)) 1)
        (Default|ResumePlayerTurn (Variables|References|GetIDI%20GM))
        (else
          (Utilities|Time|SetTimerbyFunctionName (Variables|References|GetIDI%20GM) "Start Game IDI" 2.0))))
    (:NewEnumerator1
      (if (> (Variables|/Game/Main_Game_Managers/Auction/BP_Auction_Game_Manager.BP_Auction_Game_Manager_C|GetCurrent%20Round%20Index (Variables|References|GetAuction%20GM)) 1)
        (Default|UnpauseRound (Variables|References|GetAuction%20GM))
        (else
          (Utilities|Time|SetTimerbyFunctionName (Variables|References|GetAuction%20GM) "Start Auction" 2.0))))
    (:NewEnumerator2
      (if (not (> (Variables|/Game/Main_Game_Managers/Rat_Screw/BP_Rat_Screw_Game_Manager.BP_Rat_Screw_Game_Manager_C|GetCurrent%20Round%20Index (Variables|References|GetRat%20Screw%20GM)) 1))
        (Utilities|Time|SetTimerbyFunctionName (Variables|References|GetRat%20Screw%20GM) "Begin Rat Screw" 2.0)))
    (:NewEnumerator4
      (if (not (> (Variables|/Game/Mini_Games/Darts/BP_Dart_Game_Manager.BP_Dart_Game_Manager_C|GetCurrent%20Round%20Index (Variables|References|GetDart%20Game%20Manager%20Ref)) 1))
        (Utilities|Time|SetTimerbyFunctionName (Variables|References|GetDart%20Game%20Manager%20Ref) "Begin Game" (* (Variables|/Game/Mini_Games/Darts/BP_Dart_Game_Manager.BP_Dart_Game_Manager_C|GetFade%20Time%20For%20Setup (Variables|References|GetDart%20Game%20Manager%20Ref)) 2.0))))))

(fn Pause/UnpauseGame
  (bind _pause_screen_widget (Variables|References|GetPause%20Screen%20Widget))
  (if (Game|IsGamePaused)
    ;[0 0 0] Unpause the game by adding the button prompts back to the screen, setting game paused false, hiding the mouse, setting input to game only and removing the pause widget from the viewport
    (UserInterface|Viewport|AddtoViewport (Utilities|Select :Index (Variables|CurrentGame|GetCurrent%20Playing%20Game) :NewEnumerator0 (Variables|ButtonPromptWidgets|GetIDI%20Button%20Prompt%20Widget) :NewEnumerator1 (Variables|ButtonPromptWidgets|GetAuction%20Button%20Prompt%20Widget) :NewEnumerator2 (Variables|ButtonPromptWidgets|GetRat%20Screw%20Button%20Prompt%20Widget) :NewEnumerator3 (Variables|ButtonPromptWidgets|GetPool%20Button%20Prompt%20Widget) :NewEnumerator4 (Variables|ButtonPromptWidgets|GetDarts%20Button%20Prompt%20Widget) :NewEnumerator5 (Variables|ButtonPromptWidgets|GetBar%20Button%20Prompt%20Widget)) 0)
    (Game|SetGamePaused false)
    (Variables|/Script/Engine.PlayerController|SetbShowMouseCursor (Game|GetPlayerController 0) false)
    (Input|SetInputModeGameOnly (Game|GetPlayerController 0) false)
    (Widget|RemovefromParent (Variables|References|GetPause%20Screen%20Widget))
    (else
      ;[0 0 0] Pause the game by doing the opposite of unpausing
      (Widget|RemovefromParent (Utilities|Select :Index (Variables|CurrentGame|GetCurrent%20Playing%20Game) :NewEnumerator0 (Variables|ButtonPromptWidgets|GetIDI%20Button%20Prompt%20Widget) :NewEnumerator1 (Variables|ButtonPromptWidgets|GetAuction%20Button%20Prompt%20Widget) :NewEnumerator2 (Variables|ButtonPromptWidgets|GetRat%20Screw%20Button%20Prompt%20Widget) :NewEnumerator3 (Variables|ButtonPromptWidgets|GetPool%20Button%20Prompt%20Widget) :NewEnumerator4 (Variables|ButtonPromptWidgets|GetDarts%20Button%20Prompt%20Widget) :NewEnumerator5 (Variables|ButtonPromptWidgets|GetBar%20Button%20Prompt%20Widget)))
      (Game|SetGamePaused true)
      (Variables|/Script/Engine.PlayerController|SetbShowMouseCursor (Game|GetPlayerController 0) true)
      (Input|SetInputModeGameandUI (Game|GetPlayerController 0) (Variables|References|GetPause%20Screen%20Widget) "DoNotLock" true false)
      (UserInterface|Viewport|AddtoViewport (Variables|References|GetPause%20Screen%20Widget) 0)
      (UserInterface|Animation|PlayAnimation _pause_screen_widget (Variables|/Game/UI/Non_Diegetic/Pause/WBP_Pause_Menu.WBP_Pause_Menu_C|GetPause_Menu_Wipe _pause_screen_widget) 0.0 1 "Forward" 1.0 false))))

(fn UpdateVolumeLevel
  (params (Sound%20Class :type Enum_Sound_Classes%20Enum :default "NewEnumerator0") (New%20Volume :type Float%20%28double-precision%29))
  (Utilities|Array|SetArrayElem (Variables|Default|GetVolume%20Levels) (Utilities|Select :Index Sound%20Class :NewEnumerator0 0 :NewEnumerator1 1 :NewEnumerator2 2 :NewEnumerator3 3) New%20Volume))